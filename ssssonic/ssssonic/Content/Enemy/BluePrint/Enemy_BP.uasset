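; Enemy actor that the player's BasicMouse can smash by ramming it at high speed.
; On overlap, it casts to BasicMouse and checks its GroundSpeed against a fixed threshold.
; Above the threshold, the enemy destroys itself, adds coins to the mouse, spawns a coin-burst Niagara effect and adds an audio component.
; Otherwise it calls Hit on the mouse.
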(event EventBeginPlay)

(event Collision|EventActorBeginOverlap
  (params (OtherActor :type Actor%20Object%20Reference))
  (bind _asbasic_mouse (Utilities|Casting|CastToBasicMouse OtherActor))
  (if (> (Variables|/Game/BasicMouse.BasicMouse_C|GetGroundSpeed _asbasic_mouse) 1e+03)
    (Actor|DestroyActor)
    (Variables|/Game/BasicMouse.BasicMouse_C|SetCoin _asbasic_mouse (+ (Variables|/Game/BasicMouse.BasicMouse_C|GetCoin _asbasic_mouse) 10))
    (Niagara|SpawnSystematLocation "/Game/sA_PickupSet_1/Fx/NiagaraSystems/NS_CoinBurst.NS_CoinBurst" (Transformation|GetActorLocation))
    (AddComponent|AddAudioComponent false)
    (else
      (Default|Hit _asbasic_mouse))))

(event EventTick
  (params (DeltaSeconds :type Float%20%28single-precision%29)))

(fn ConstructionScript)