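; BP_DC_MagicLink is a visual effect Blueprint in the audio demo assets that pairs a main particle system with a whirlwind lightning particle effect.
; ActivateAll restarts both particle components with a reset, and DeactivateAll deactivates both.
; The construction script applies the LightningScale variable as the relative scale of the lightning component.
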(event Custom|ActivateAll
  (Components|Activation|Activate (Variables|Emitter|GetParticleSystemComponent) true)
  (Components|Activation|Activate (Variables|Default|GetP_Whirlwind_Lightning_01) true))

(event Custom|DeactivateAll
  (Components|Activation|Deactivate (Variables|Emitter|GetParticleSystemComponent))
  (Components|Activation|Deactivate (Variables|Default|GetP_Whirlwind_Lightning_01)))

(fn ConstructionScript
  (Transformation|SetRelativeScale3D (Variables|Default|GetP_Whirlwind_Lightning_01) (Variables|Default|GetLightningScale)))