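; BP_DC_MagicCrate is an interactive crate that plays a scaling effect and then explodes when triggered with the E key.
; Overlapping the Box opens a gate for the key input, and leaving closes it, with no filter on the overlapping actor.
; A timeline multiplies the cached BeginPlay world scales of P01, P02 and P03, then activates Explosion and deactivates all three when finished.
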(event OnComponentBeginOverlap(Box)
  (params (OverlappedComponent :type Primitive%20Component%20Object%20Reference) (OtherActor :type Actor%20Object%20Reference) (OtherComp :type Primitive%20Component%20Object%20Reference) (OtherBodyIndex :type Integer) (bFromSweep :type Boolean) (SweepResult :type Hit%20Result%20Structure%20%28by%20ref%29))
  (Utilities|FlowControl|Gate true) ; enters at Open
)

(event OnComponentEndOverlap(Box)
  (params (OverlappedComponent :type Primitive%20Component%20Object%20Reference) (OtherActor :type Actor%20Object%20Reference) (OtherComp :type Primitive%20Component%20Object%20Reference) (OtherBodyIndex :type Integer))
  (Utilities|FlowControl|Gate true) ; enters at Close
)

(event EventBeginPlay
  (Variables|Default|SetP01_Scale (Transformation|GetWorldScale (Variables|Default|GetP01)))
  (Variables|Default|SetP02_Scale (Transformation|GetWorldScale (Variables|Default|GetP02)))
  (Variables|Default|SetP03_Scale (Transformation|GetWorldScale (Variables|Default|GetP03))))

(event Input|KeyboardEvents|E
  (params (Key :type Key%20Structure :default "None"))
  (:Pressed
    (Utilities|FlowControl|Gate true
      (:Exit
        (bind _newtrack_0 (Timeline|Timeline_0 PlayFromStart)
          (:Update
            (Transformation|SetWorldScale3D (Variables|Default|GetP01) (* (Variables|Default|GetP01_Scale) _newtrack_0))
            (Transformation|SetWorldScale3D (Variables|Default|GetP02) (* (Variables|Default|GetP02_Scale) _newtrack_0))
            (Transformation|SetWorldScale3D (Variables|Default|GetP03) (* (Variables|Default|GetP03_Scale) _newtrack_0)))
          (:Finished
            (Components|Activation|Activate (Variables|Default|GetExplosion) true)
            (Components|Activation|Deactivate (Variables|Default|GetP01))))))))

(fn ConstructionScript)