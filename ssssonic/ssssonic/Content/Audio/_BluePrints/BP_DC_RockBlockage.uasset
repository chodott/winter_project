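; Rock blockage the player clears with a spell by pressing E inside a trigger box on either side.
; Overlaps open input gates; while Active, E plays a sound, toggles two audio volumes in that side's direction and casts its spell.
; Each mirrored sequence turns a spell effect toward the player, scales it by timeline, damages the destructible rock, then shrinks and spins it under beam effects before destroying it and clearing Active.
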(event OnComponentBeginOverlap(Box)
  (params (OverlappedComponent :type Primitive%20Component%20Object%20Reference) (OtherActor :type Actor%20Object%20Reference) (OtherComp :type Primitive%20Component%20Object%20Reference) (OtherBodyIndex :type Integer) (bFromSweep :type Boolean) (SweepResult :type Hit%20Result%20Structure%20%28by%20ref%29))
  ;[1 1 1] Activate
  (if (== 0 (Game|GetPlayerCharacter 0))
    (Utilities|FlowControl|Gate true) ; enters at Open
  ))

(event OnComponentEndOverlap(Box)
  (params (OverlappedComponent :type Primitive%20Component%20Object%20Reference) (OtherActor :type Actor%20Object%20Reference) (OtherComp :type Primitive%20Component%20Object%20Reference) (OtherBodyIndex :type Integer))
  ;[1 1 1] Activate
  (if (== 0 (Game|GetPlayerCharacter 0))
    (Utilities|FlowControl|Gate true) ; enters at Close
  ))

(event OnComponentBeginOverlap(Box1)
  (params (OverlappedComponent :type Primitive%20Component%20Object%20Reference) (OtherActor :type Actor%20Object%20Reference) (OtherComp :type Primitive%20Component%20Object%20Reference) (OtherBodyIndex :type Integer) (bFromSweep :type Boolean) (SweepResult :type Hit%20Result%20Structure%20%28by%20ref%29))
  ;[1 1 1] Activate
  (Utilities|FlowControl|Gate true) ; enters at Open
)

(event OnComponentEndOverlap(Box1)
  (params (OverlappedComponent :type Primitive%20Component%20Object%20Reference) (OtherActor :type Actor%20Object%20Reference) (OtherComp :type Primitive%20Component%20Object%20Reference) (OtherBodyIndex :type Integer))
  ;[1 1 1] Activate
  (Utilities|FlowControl|Gate true) ; enters at Close
)

(event Custom|CastSpellReverse
  (bind _returnvalue (Game|GetPlayerCharacter 0))
  (bind _rock (Variables|Default|GetRock))
  (bind _rock_2 (Variables|Default|GetRock))
  (bind _rock_rotation (Variables|Default|GetRock%20Rotation))
  (bind _spell1 (Variables|Default|GetSpell1))
  (bind _returnvalue_2 (Transformation|GetWorldLocation _spell1))
  (bind _returnvalue_3 (Transformation|GetActorLocation _returnvalue))
  (bind _returnvalue_4 (Math|Rotator|FindLookatRotation _returnvalue_2 _returnvalue_3))
  ;[1 1 1] Start system when coming from oppoiste direction
  (Transformation|SetWorldRotation (Variables|Default|GetSpell1) (Math|Rotator|MakeRotator (.roll _returnvalue_4) (+ (.pitch _returnvalue_4) 9e+01) (.yaw _returnvalue_4)) false false)
  (Components|Activation|Activate (Variables|Default|GetSpell1) false)
  (bind _newtrack_0 (Timeline|Timeline_3 PlayFromStart)
    (:Update
      (Transformation|SetWorldScale3D (Variables|Default|GetSpell1) (* (Variables|Default|GetSpellSize) _newtrack_0)))
    (:Finished
      (Components|Activation|Activate (Variables|Default|GetSparkle1) false)
      (Utilities|FlowControl|Delay 0.5)
      (Components|Activation|Deactivate (Variables|Default|GetSpell1))
      (Components|Activation|Activate (Variables|Default|GetExplosion1) false)
      (Class|DestructibleComponent|ApplyDamage (Variables|/Script/ApexDestruction.DestructibleActor|GetDestructibleComponent _rock_2) 5e+02 (Transformation|GetActorLocation _rock_2) (Transformation|GetActorForwardVector (Game|GetPlayerCharacter 0)) 1e+04)
      (Components|Activation|Activate (Variables|Default|GetP_Charge_Target_Beam_Ice1) true)
      (Utilities|FlowControl|Delay 2.0)
      (bind _newtrack_0_2 (Timeline|Timeline_2 PlayFromStart)
        (:Update
          (Transformation|SetWorldScale3D (Variables|/Script/Engine.Actor|GetRootComponent _rock) (* (Variables|Default|GetRockSize) _newtrack_0_2))
          (Transformation|SetWorldRotation (Variables|/Script/ApexDestruction.DestructibleActor|GetDestructibleComponent _rock) (Math|Rotator|MakeRotator (.roll _rock_rotation) (.pitch _rock_rotation) (+ (.yaw _rock_rotation) (* (- 1.0 _newtrack_0_2) 7.2e+02))) false false))
        (:Finished
          (Actor|DestroyActor (Variables|Default|GetRock))
          (Components|Activation|Deactivate (Variables|Default|GetP_Charge_Target_Beam_Ice1))
          (Variables|Default|SetActive false))))))

(event Custom|CastSpell
  (bind _returnvalue (Game|GetPlayerCharacter 0))
  (bind _spell (Variables|Default|GetSpell))
  (bind _rock (Variables|Default|GetRock))
  (bind _rock_2 (Variables|Default|GetRock))
  (bind _rock_rotation (Variables|Default|GetRock%20Rotation))
  (bind _returnvalue_2 (Transformation|GetActorLocation _returnvalue))
  (bind _returnvalue_3 (Transformation|GetWorldLocation _spell))
  (bind _returnvalue_4 (Math|Rotator|FindLookatRotation _returnvalue_3 _returnvalue_2))
  ;[1 1 1] Start system
  (Transformation|SetWorldRotation (Variables|Default|GetSpell) (Math|Rotator|MakeRotator (.roll _returnvalue_4) (+ (.pitch _returnvalue_4) 9e+01) (.yaw _returnvalue_4)) false false)
  (Components|Activation|Activate (Variables|Default|GetSpell) false)
  (bind _newtrack_0 (Timeline|Timeline_1 PlayFromStart)
    (:Update
      (Transformation|SetWorldScale3D (Variables|Default|GetSpell) (* (Variables|Default|GetSpellSize) _newtrack_0)))
    (:Finished
      (Components|Activation|Activate (Variables|Default|GetSparkle) false)
      (Utilities|FlowControl|Delay 0.5)
      (Components|Activation|Deactivate (Variables|Default|GetSpell))
      (Components|Activation|Activate (Variables|Default|GetExplosion) false)
      (Class|DestructibleComponent|ApplyDamage (Variables|/Script/ApexDestruction.DestructibleActor|GetDestructibleComponent _rock) 5e+02 (Transformation|GetActorLocation _rock) (Transformation|GetActorForwardVector (Game|GetPlayerCharacter 0)) 1e+04)
      (Components|Activation|Activate (Variables|Default|GetP_Charge_Target_Beam_Ice1) true)
      (Utilities|FlowControl|Delay 2.0)
      (bind _newtrack_0_2 (Timeline|Timeline_0 PlayFromStart)
        (:Update
          (Transformation|SetWorldScale3D (Variables|/Script/Engine.Actor|GetRootComponent _rock_2) (* (Variables|Default|GetRockSize) _newtrack_0_2))
          (Transformation|SetWorldRotation (Variables|/Script/ApexDestruction.DestructibleActor|GetDestructibleComponent _rock_2) (Math|Rotator|MakeRotator (.roll _rock_rotation) (.pitch _rock_rotation) (+ (.yaw _rock_rotation) (* (- 1.0 _newtrack_0_2) 7.2e+02))) false false))
        (:Finished
          (Actor|DestroyActor (Variables|Default|GetRock))
          (Components|Activation|Deactivate (Variables|Default|GetP_Charge_Target_Beam_Ice1))
          (Variables|Default|SetActive false))))))

(event EventBeginPlay
  (bind _rock (Variables|Default|GetRock))
  ;[1 1 1] set up
  (Variables|Default|SetRockSize (Transformation|GetWorldScale (Variables|/Script/Engine.Actor|GetRootComponent _rock)))
  (Variables|Default|SetRock%20Rotation (Transformation|GetWorldRotation (Variables|/Script/Engine.Actor|GetRootComponent _rock))))

(event Input|KeyboardEvents|E
  (params (Key :type Key%20Structure :default "None"))
  ;[1 1 1] Activate
  (:Pressed
    (Utilities|FlowControl|Gate true
      (:Exit
        (if (Variables|Default|GetActive)
          (CallFunction|CastSpellReverse)
          (Audio|PlaySound2D "/Game/Audio/Magic/Rock_Blockage.Rock_Blockage" 0.6 1.0 0.0 0 0)
          (Class|AudioVolume|SetEnabled (Variables|Default|GetAudio_Volume) true)
          (Class|AudioVolume|SetEnabled (Variables|Default|GetAudio_Volume_2) false))))))

(event Input|KeyboardEvents|E
  (params (Key :type Key%20Structure :default "None"))
  ;[1 1 1] Activate
  (:Pressed
    (Utilities|FlowControl|Gate true
      (:Exit
        (if (Variables|Default|GetActive)
          (CallFunction|CastSpell)
          (Audio|PlaySound2D "/Game/Audio/Magic/Rock_Blockage.Rock_Blockage" 0.6 1.0 0.0 0 0)
          (Class|AudioVolume|SetEnabled (Variables|Default|GetAudio_Volume) false)
          (Class|AudioVolume|SetEnabled (Variables|Default|GetAudio_Volume_2) true))))))

(fn ConstructionScript)