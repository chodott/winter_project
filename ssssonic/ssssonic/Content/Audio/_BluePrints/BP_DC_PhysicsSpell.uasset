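; Physics spell actor that handles the charge and release effects and sounds for a spell cast by the first-person character.
; While charging, Tick follows the player's SpellSocket with a height offset, matches camera rotation and grows ChargingFX up to a clamped size.
; Release deactivates the effect, plays a fire sound, fades out the charge sound and destroys the actor after a short delay.
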(event Custom|ChargeSpell
  ;[1 1 1] Start charging
  (Transformation|SetWorldScale3D (Variables|Default|GetChargingFX) (Variables|Default|GetInitialScale))
  (Actor|Tick|SetActorTickEnabled true)
  (Components|Activation|Activate (Variables|Default|GetChargingFX) false)
  (Variables|Default|SetCharging true)
  (bind _returnvalue (Audio|SpawnSoundatLocation "/Game/Audio/Magic/Magic_Bolt_Simple.Magic_Bolt_Simple" (Transformation|GetActorLocation self) "0, 0, 0" 1.0 1.0 0.0 0 0)))

(event Custom|ReleaseSpell
  ;[1 1 1] Release spell
  (Components|Activation|Deactivate (Variables|Default|GetChargingFX))
  (Variables|Default|SetCharging false)
  (bind _asfirst_person_character (Utilities|Casting|CastToFirstPersonCharacter (Game|GetPlayerCharacter 0)))
  (Audio|PlaySoundatLocation "/Game/Audio/Magic/Magic_bolt_spell_fire.Magic_bolt_spell_fire" (Transformation|GetActorLocation self) "0, 0, 0" 0.6 1.0 0.0 0 0 0)
  (Audio|Components|Audio|FadeOut (stale Custom|ChargeSpell _returnvalue) 0.2 0.0 :!class /Script/Engine.AudioComponent)
  (Utilities|FlowControl|Delay 2.0)
  (Actor|DestroyActor))

(event EventTick
  (params (DeltaSeconds :type Float%20%28single-precision%29))
  ;[1 1 1] Charge spell
  (if (Variables|Default|GetCharging)
    (bind _asfirst_person_character (Utilities|Casting|CastToFirstPersonCharacter (Game|GetPlayerCharacter 0)))
    (Transformation|SetActorRotation (Transformation|GetWorldRotation (Variables|/Game/FirstPersonBP/Blueprints/FirstPersonCharacter.FirstPersonCharacter_C|GetFirstPersonCamera _asfirst_person_character)))
    (Transformation|SetActorLocation (+ (Transformation|GetWorldLocation (Variables|/Game/FirstPersonBP/Blueprints/FirstPersonCharacter.FirstPersonCharacter_C|GetSpellSocket _asfirst_person_character)) (Math|Vector|MakeVector 0.0 0.0 (Variables|Default|GetHeightOffsetCharge))) false false)
    (Transformation|SetWorldScale3D (Variables|Default|GetChargingFX) (Math|Vector|ClampVectorSize (* (Transformation|GetWorldScale (Variables|Default|GetChargingFX)) (Variables|Default|GetChargeScalingFactor)) 0.0 0.7))))

(event EventBeginPlay
  ;[1 1 1] Get starting scale
  (Variables|Default|SetInitialScale (Transformation|GetWorldScale (Variables|Default|GetChargingFX))))

(fn ConstructionScript)