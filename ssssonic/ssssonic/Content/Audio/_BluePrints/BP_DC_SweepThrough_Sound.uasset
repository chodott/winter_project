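; BP_DC_SweepThrough_Sound is a one-shot audio actor that moves a sound through the level along its forward vector.
; Shortly after BeginPlay it applies the configured sound and attenuation to its audio component and plays it.
; Tick advances the actor by Speed each frame without scaling by delta time, so the sweep rate depends on frame rate.
; When playback finishes, the actor disables tick and destroys itself.
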(event Custom|OnAudioFinished_Event_0
  ;[1 1 1] set up
  (Actor|Tick|SetActorTickEnabled false)
  (Actor|DestroyActor))

(event EventBeginPlay
  (bind _audio (Variables|Default|GetAudio))
  ;[1 1 1] set up
  (Utilities|FlowControl|Delay 0.2)
  (Audio|Components|Audio|SetSound _audio (Variables|Default|GetSound))
  (Variables|/Script/Engine.AudioComponent|SetAttenuationSettings _audio (Variables|Default|GetAttenuation))
  (Audio|Components|Audio|Play _audio 0.0)
  (EventDispatchers|AssignOnAudioFinished (Variables|Default|GetAudio) (delegate Custom|OnAudioFinished_Event_0)))

(event EventTick
  (params (DeltaSeconds :type Float%20%28single-precision%29))
  (bind _returnvalue (Transformation|GetActorLocation))
  (bind _returnvalue_2 (Transformation|GetActorForwardVector))
  (bind _speed (Variables|Default|GetSpeed))
  (bind _returnvalue_3 (* _returnvalue_2 _speed))
  (bind _returnvalue_4 (+ _returnvalue _returnvalue_3))
  ;[1 1 1] set location
  (Transformation|SetActorLocation _returnvalue_4 false false)
  (Development|PrintString (Utilities|String|ToString(Vector) _returnvalue_4) false true "(R=0.000000,G=0.660000,B=1.000000,A=1.000000)" DeltaSeconds))

(fn ConstructionScript)