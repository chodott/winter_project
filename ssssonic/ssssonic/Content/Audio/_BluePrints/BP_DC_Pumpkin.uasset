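; Destructible pumpkin Blueprint that plays a fruit drop sound and breaks on impact.
; Until a fracture sets Broken, a hit on a SplatPlatform-tagged component passes through a DoOnce to spawn the sound at the hit point and apply damage along the hit normal.
; Hits on Pot-tagged components reach a DoOnceMultiInput with no further action shown.
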(event OnComponentFracture(Destructible)
  (params (HitPoint :type Vector%20%28by%20ref%29 :default "0, 0, 0") (HitDirection :type Vector%20%28by%20ref%29 :default "0, 0, 0"))
  ;[1 1 1] set broken
  (Variables|Default|SetBroken true))

(event OnComponentHit(Destructible)
  (params (HitComponent :type Primitive%20Component%20Object%20Reference) (OtherActor :type Actor%20Object%20Reference) (OtherComp :type Primitive%20Component%20Object%20Reference) (NormalImpulse :type Vector :default "0, 0, 0") (Hit :type Hit%20Result%20Structure%20%28by%20ref%29))
  (bind (_bblockinghit _binitialoverlap _time _distance _location _impactpoint _normal) (Collision|BreakHitResult Hit))
  ;[1 1 1] play sound on hit event
  (if (not (Variables|Default|GetBroken))
    (if (Components|ComponentHasTag OtherComp "SplatPlatform")
      (Utilities|FlowControl|DoOnce false
        (:Completed
          (Audio|SpawnSoundatLocation "/Game/Audio/Props/Fruit_Drop/as_pr_Fruit_Drop_01.as_pr_Fruit_Drop_01" _location "0, 0, 0" 1.0 1.0 0.0 0 0)
          (Class|DestructibleComponent|ApplyDamage (Variables|Default|GetDestructible) 5.0 _location _normal 0.0)))
      (else
        ;[1 1 1] Landing in Pot
        (if (Components|ComponentHasTag OtherComp "Pot")
          (|DoOnceMultiInput))))))

(fn ConstructionScript)