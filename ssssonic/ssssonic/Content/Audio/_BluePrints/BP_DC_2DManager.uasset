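; Manager Blueprint that toggles the player between first-person 3D and 2D play.
; Each player overlap of the entrance trigger alternates modes through a FlipFlop, hiding the change behind a delayed camera and audio fade.
; Going 2D faces the character toward ExitTarget, stores that direction, locks free camera and enables the 2D camera.
; Returning restores first-person view and free camera, with control yaw opposite the character's facing.
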(event OnActorBeginOverlap(2DEntranceTrigger)
  (params (OverlappedActor :type Actor%20Object%20Reference) (OtherActor :type Actor%20Object%20Reference))
  ;[1 1 1] toggle between 2D & 3D
  (if (== OtherActor (Game|GetPlayerCharacter 0))
    (Utilities|FlowControl|FlipFlop
      (:A
        (CallFunction|Switchto2D))
      (:B
        (CallFunction|Switchto3D)))))

(event Custom|SwitchTo2D
  (bind _returnvalue (Game|GetPlayerCharacter 0))
  (bind _returnvalue_2 (Game|GetPlayerCharacter 0))
  (bind _returnvalue_3 (Transformation|GetActorRotation _returnvalue))
  ;[1 1 1] Switch to 2D
  (CameraFades|StartCameraFade :self (Variables|/Script/Engine.PlayerController|GetPlayerCameraManager (Game|GetPlayerController 0)) :ToAlpha 1.0 :Duration 2.0 :bShouldFadeAudio true :bHoldWhenFinished true)
  (Utilities|FlowControl|Delay 3.0)
  (Transformation|SetActorRotation _returnvalue (Math|Rotator|MakeRotator (.roll _returnvalue_3) (.pitch _returnvalue_3) (.yaw (Math|Rotator|FindLookatRotation (Transformation|GetActorLocation _returnvalue) (Transformation|GetActorLocation (Variables|Default|GetExitTarget))))))
  (bind _asfirst_person_character (Utilities|Casting|CastToFirstPersonCharacter _returnvalue_2))
  (Variables|/Game/FirstPersonBP/Blueprints/FirstPersonCharacter.FirstPersonCharacter_C|Set2D_Direction _asfirst_person_character (Transformation|GetActorForwardVector _returnvalue_2))
  (Variables|/Game/FirstPersonBP/Blueprints/FirstPersonCharacter.FirstPersonCharacter_C|SetIn2D _asfirst_person_character true)
  (Variables|/Game/FirstPersonBP/Blueprints/FirstPersonCharacter.FirstPersonCharacter_C|SetAllowFreeCamera _asfirst_person_character false)
  (Default|2DCameraon _asfirst_person_character)
  (CameraFades|StartCameraFade :self (Variables|/Script/Engine.PlayerController|GetPlayerCameraManager (Game|GetPlayerController 0)) :FromAlpha 1.0 :Duration 2.0 :bShouldFadeAudio true))

(event Custom|SwitchTo3D
  (bind _returnvalue (Game|GetPlayerCharacter 0))
  (bind _returnvalue_2 (Transformation|GetActorRotation _returnvalue))
  ;[1 1 1] Switch to 3D
  (CameraFades|StartCameraFade :self (Variables|/Script/Engine.PlayerController|GetPlayerCameraManager (Game|GetPlayerController 0)) :ToAlpha 1.0 :Duration 2.0 :bShouldFadeAudio true :bHoldWhenFinished true)
  (Utilities|FlowControl|Delay 3.0)
  (bind _asfirst_person_character (Utilities|Casting|CastToFirstPersonCharacter (Game|GetPlayerCharacter 0)))
  (Variables|/Game/FirstPersonBP/Blueprints/FirstPersonCharacter.FirstPersonCharacter_C|SetIn2D _asfirst_person_character false)
  (Default|ResettoFirstPerson _asfirst_person_character)
  (Variables|/Game/FirstPersonBP/Blueprints/FirstPersonCharacter.FirstPersonCharacter_C|SetAllowFreeCamera _asfirst_person_character true)
  (Pawn|SetControlRotation (Game|GetPlayerController 0) (Math|Rotator|MakeRotator (.roll _returnvalue_2) (.pitch _returnvalue_2) (- (.yaw _returnvalue_2) 1.8e+02)))
  (CameraFades|StartCameraFade :self (Variables|/Script/Engine.PlayerController|GetPlayerCameraManager (Game|GetPlayerController 0)) :FromAlpha 1.0 :Duration 2.0 :bShouldFadeAudio true :bHoldWhenFinished true))

(fn ConstructionScript)