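; Interactive music box prop that the player switches on and off with the E key while standing inside its trigger box.
; Box1 overlaps with the player character open and close a Gate on the key press, which feeds a FlipFlop alternating Play and Stop.
; Play and Stop toggle a RotatingMovement component bound to the Cylinder at BeginPlay and fade the music in or out.
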(event OnComponentBeginOverlap(Box1)
  (params (OverlappedComponent :type Primitive%20Component%20Object%20Reference) (OtherActor :type Actor%20Object%20Reference) (OtherComp :type Primitive%20Component%20Object%20Reference) (OtherBodyIndex :type Integer) (bFromSweep :type Boolean) (SweepResult :type Hit%20Result%20Structure%20%28by%20ref%29))
  ;[1 1 1] On / off
  (if (== OtherActor (Game|GetPlayerCharacter 0))
    (Utilities|FlowControl|Gate true) ; enters at Open
  ))

(event OnComponentEndOverlap(Box1)
  (params (OverlappedComponent :type Primitive%20Component%20Object%20Reference) (OtherActor :type Actor%20Object%20Reference) (OtherComp :type Primitive%20Component%20Object%20Reference) (OtherBodyIndex :type Integer))
  ;[1 1 1] On / off
  (if (== OtherActor (Game|GetPlayerCharacter 0))
    (Utilities|FlowControl|Gate true) ; enters at Close
  ))

(event Custom|Play
  ;[1 1 1] play / stop
  (Components|Activation|SetActive (Variables|Default|GetRotatingMovement) true false)
  (Audio|Components|Audio|FadeIn (Variables|Default|GetMusic) 1.0 1.0 0.0 :!class /Script/Engine.AudioComponent))

(event Custom|Stop
  ;[1 1 1] play / stop
  (Components|Activation|SetActive (Variables|Default|GetRotatingMovement) false false)
  (Audio|Components|Audio|FadeOut (Variables|Default|GetMusic) 1.0 0.0 :!class /Script/Engine.AudioComponent))

(event EventBeginPlay
  ;[1 1 1] set up
  (Components|Movement|SetUpdatedComponent (Variables|Default|GetRotatingMovement) (Variables|Default|GetCylinder)))

(event Input|KeyboardEvents|E
  (params (Key :type Key%20Structure :default "None"))
  ;[1 1 1] On / off
  (:Pressed
    (Utilities|FlowControl|Gate true
      (:Exit
        (Utilities|FlowControl|FlipFlop
          (:A
            (CallFunction|Play))
          (:B
            (CallFunction|Stop)))))))

(fn ConstructionScript)