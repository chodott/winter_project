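; Trigger actor for an "isolation spell" that toggles a post-process effect and exterior audio muting when the player presses E inside it.
; Player overlap opens and closes a Gate on the E key, so the spell only fires while in range.
; Each press plays the spell sound, then a FlipFlop waits two seconds before switching the PostProcessVolume and fading the AudioVolume's exterior volume out or back in.
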(event Collision|EventActorBeginOverlap
  (params (OtherActor :type Actor%20Object%20Reference))
  (bind _audio_volume (Variables|Default|GetAudio_Volume))
  (bind _postprocessvolume (Variables|Default|GetPostProcessVolume))
  (if (== OtherActor (Game|GetPlayerCharacter 0))
    (Utilities|FlowControl|Gate true) ; enters at Open
  ))

(event Collision|EventActorEndOverlap
  (params (OtherActor :type Actor%20Object%20Reference))
  (bind _audio_volume (Variables|Default|GetAudio_Volume))
  (bind _postprocessvolume (Variables|Default|GetPostProcessVolume))
  (if (== OtherActor (Game|GetPlayerCharacter 0))
    (Utilities|FlowControl|Gate true) ; enters at Close
  ))

(event Input|KeyboardEvents|E
  (params (Key :type Key%20Structure :default "None"))
  (bind _audio_volume (Variables|Default|GetAudio_Volume))
  (bind _postprocessvolume (Variables|Default|GetPostProcessVolume))
  (:Pressed
    (Utilities|FlowControl|Gate true
      (:Exit
        (Audio|PlaySound2D "/Game/Audio/Magic/Isolation_spell.Isolation_spell" 1.0 1.0 0.0 0 0)
        (Utilities|FlowControl|FlipFlop
          (:A
            (Utilities|FlowControl|Delay 2.0)
            (Variables|/Script/Engine.PostProcessVolume|SetbEnabled _postprocessvolume true)
            (Class|AudioVolume|SetInteriorSettings _audio_volume (Utilities|Struct|MakeInteriorSettings 0.0 0.5)))
          (:B
            (Utilities|FlowControl|Delay 2.0)
            (Variables|/Script/Engine.PostProcessVolume|SetbEnabled _postprocessvolume false)
            (Class|AudioVolume|SetInteriorSettings _audio_volume (Utilities|Struct|MakeInteriorSettings 1.0 0.5))))))))

(fn ConstructionScript)