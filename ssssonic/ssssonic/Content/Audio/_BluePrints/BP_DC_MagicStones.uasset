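; Magic stone actor that reacts once to a sufficiently powerful magic bolt and counts toward a spell.
; When a BP_DC_MagicBolt hits its mesh with Power at or above the threshold, it activates particles, plays a fire sound and increments the stone count on SpellBP.
; A gate then closes so each stone triggers only once.
; The configurable static mesh is applied in both the construction script and BeginPlay.
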(event OnComponentHit(StaticMeshComponent)
  (params (HitComponent :type Primitive%20Component%20Object%20Reference) (OtherActor :type Actor%20Object%20Reference) (OtherComp :type Primitive%20Component%20Object%20Reference) (NormalImpulse :type Vector :default "0, 0, 0") (Hit :type Hit%20Result%20Structure%20%28by%20ref%29))
  ;[1 1 1] activate
  (Utilities|FlowControl|Gate false :!label _label
    (:Exit
      (if (== (Utilities|GetClass OtherActor) "/Game/Audio/_BluePrints/BP_DC_MagicBolt.BP_DC_MagicBolt_C")
        (bind _asbp_dc_magic_bolt (Utilities|Casting|CastToBP_DC_MagicBolt OtherActor))
        (if (>= (Variables|/Game/Audio/_BluePrints/BP_DC_MagicBolt.BP_DC_MagicBolt_C|GetPower _asbp_dc_magic_bolt) (Variables|Default|GetPowerThreshold))
          (Components|Activation|Activate (Variables|Default|GetParticleSystem) false)
          (Audio|Components|Audio|Play (Variables|Default|GetMagic_Bolt_Fire-001) 0.0)
          (Default|IncrementStones (Variables|Default|GetSpell_BP))
          (goto _label Close))))))

(event EventBeginPlay
  ;[1 1 1] set up
  (Components|StaticMesh|SetStaticMesh (Variables|Debug|GetStaticMeshComponent) (Variables|Default|GetStaticMesh)))

(fn ConstructionScript
  (Components|StaticMesh|SetStaticMesh (Variables|Debug|GetStaticMeshComponent) (Variables|Default|GetStaticMesh)))