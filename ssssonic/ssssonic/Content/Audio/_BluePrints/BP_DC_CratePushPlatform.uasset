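; Audio demo platform where the player spawns a scraping physics crate and pushes it with a charged spell.
; Trigger box overlap opens and closes gates on the inputs, so they only work while the player is inside.
; E breaks any existing crate with a wood burst and spawns a replacement.
; Left mouse hold time sets the crate's thruster strength, fired briefly on release along a direction derived from player yaw.
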(event OnComponentBeginOverlap(TriggerBox)
  (params (OverlappedComponent :type Primitive%20Component%20Object%20Reference) (OtherActor :type Actor%20Object%20Reference) (OtherComp :type Primitive%20Component%20Object%20Reference) (OtherBodyIndex :type Integer) (bFromSweep :type Boolean) (SweepResult :type Hit%20Result%20Structure%20%28by%20ref%29))
  ;[1 1 1] Spawn crate
  (if (== OtherActor (Game|GetPlayerCharacter 0))
    (Utilities|FlowControl|Sequence
      (:then_0
        (Utilities|FlowControl|Gate true) ; enters at Open
      )
      (:then_1
        ;[1 1 1] Charge spell & release
        (Utilities|FlowControl|Gate true) ; enters at Open
      )
      (:then_2
        (Utilities|FlowControl|Gate true) ; enters at Open
      ))))

(event OnComponentEndOverlap(TriggerBox)
  (params (OverlappedComponent :type Primitive%20Component%20Object%20Reference) (OtherActor :type Actor%20Object%20Reference) (OtherComp :type Primitive%20Component%20Object%20Reference) (OtherBodyIndex :type Integer))
  ;[1 1 1] Spawn crate
  (if (== OtherActor (Game|GetPlayerCharacter 0))
    (Utilities|FlowControl|Sequence
      (:then_0
        (Utilities|FlowControl|Gate true) ; enters at Close
      )
      (:then_1
        ;[1 1 1] Charge spell & release
        (Utilities|FlowControl|Gate true) ; enters at Close
      )
      (:then_2
        (Utilities|FlowControl|Gate true) ; enters at Close
      ))))

(event Input|MouseEvents|LeftMouseButton
  (params (Key :type Key%20Structure :default "None"))
  (bind _boxtopush (Variables|Default|GetBoxToPush))
  (bind _boxtopush_2 (Variables|Default|GetBoxToPush))
  (bind _physicsthruster (Variables|/Game/Audio/_BluePrints/BP_DC_PhysicsBox_Scraping.BP_DC_PhysicsBox_Scraping_C|GetPhysicsThruster _boxtopush_2))
  ;[1 1 1] Charge spell & release
  (:Pressed
    (Utilities|FlowControl|Gate true
      (:Exit
        (Variables|Default|SetMouseDownTime (Utilities|Time|GetTimeSeconds))
        (bind _returnvalue (Game|SpawnActorfromClass "/Game/Audio/_BluePrints/BP_DC_PhysicsSpell.BP_DC_PhysicsSpell_C" (Transformation|GetActorTransform) "Undefined" 0 0))
        (Variables|Default|SetPhysicsSpell _returnvalue)
        (Default|ChargeSpell (Variables|Default|GetPhysicsSpell)))))
  (:Released
    (Utilities|FlowControl|Gate true
      (:Exit
        (Utilities|IsValid (Variables|Default|GetBoxToPush)
          (:Is%20Valid
            (Transformation|SetWorldRotation (Variables|/Game/Audio/_BluePrints/BP_DC_PhysicsBox_Scraping.BP_DC_PhysicsBox_Scraping_C|GetPhysicsThruster (Variables|Default|GetBoxToPush)) (Math|Rotator|MakeRotator 0.0 0.0 (- (.yaw (Transformation|GetActorRotation (Game|GetPlayerCharacter 0))) 1.8e+02)) false false)
            (Variables|/Script/Engine.PhysicsThrusterComponent|SetThrustStrength _physicsthruster (Math|Float|MapRangeClamped (- (Utilities|Time|GetTimeSeconds) (Variables|Default|GetMouseDownTime)) 0.0 2.0 1e+02 1e+06))
            (Components|Activation|Activate _physicsthruster true)
            (Utilities|IsValid (Variables|Default|GetPhysicsSpell)
              (:Is%20Valid
                (Default|ReleaseSpell (Variables|Default|GetPhysicsSpell))
                (Utilities|FlowControl|Delay 0.5)
                (Utilities|IsValid _boxtopush
                  (:Is%20Valid
                    (Components|Activation|Deactivate (Variables|/Game/Audio/_BluePrints/BP_DC_PhysicsBox_Scraping.BP_DC_PhysicsBox_Scraping_C|GetPhysicsThruster _boxtopush))))))))))))

(event Input|KeyboardEvents|E
  (params (Key :type Key%20Structure :default "None"))
  ;[1 1 1] Spawn crate
  (:Pressed
    (Utilities|FlowControl|Gate true
      (:Exit
        (if (Utilities|IsValid (Variables|Default|GetBoxToPush))
          (Effects|SpawnEmitteratLocation "/Game/InfinityBladeEffects/Effects/FX_Breakables/barrel/P_BarrelBreak_Wood.P_BarrelBreak_Wood" (Transformation|GetWorldLocation (Variables|/Game/Audio/_BluePrints/BP_DC_PhysicsBox_Scraping.BP_DC_PhysicsBox_Scraping_C|GetStaticMesh (Variables|Default|GetBoxToPush))) "0, 0, 0" "2.000000,2.000000,2.000000")
          (Actor|DestroyActor (Variables|Default|GetBoxToPush)))
        (Components|Activation|Activate (Variables|Default|GetP_Summon_Child_Startup) false)
        (Utilities|FlowControl|Delay 0.5)
        (bind _returnvalue (Game|SpawnActorfromClass "/Game/Audio/_BluePrints/BP_DC_PhysicsBox_Scraping.BP_DC_PhysicsBox_Scraping_C" (Transformation|GetWorldTransform (Variables|Default|GetSpawnPoint)) "Undefined" 0 0))
        (Variables|Default|SetBoxToPush _returnvalue)))))

(fn ConstructionScript)