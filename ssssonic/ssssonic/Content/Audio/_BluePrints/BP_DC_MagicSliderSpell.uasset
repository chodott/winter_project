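; BP_DC_MagicSliderSpell is a magic spell effect Blueprint that switches a group of particle systems on and off.
; Its TurnOn event activates four particle components without a reset, including fake blue light and level-up effects.
; Its TurnOff event deactivates the same components.
; The Blueprint has no other logic, and its construction script is empty.
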(event Custom|TurnOn
  ;[1 1 1] turn on
  (Components|Activation|Activate (Variables|Emitter|GetParticleSystemComponent) false))

(event Custom|TurnOff
  ;[1 1 1] turn off
  (Components|Activation|Deactivate (Variables|Emitter|GetParticleSystemComponent)))

(fn ConstructionScript)