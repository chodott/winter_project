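; Interactive torch-slider puzzle that raises and activates a magic stone when solved.
; Pressing E inside the box, if unlocked, toggles a fixed camera with cursor control; mouse drags slide the torch along X.
; Torch position drives curves scaling the spell particles and two audio layers.
; Notch overlaps advance ordered stages; holding the last notch triggers FinalStage by timer, whose timeline lifts the stone, then exits puzzle mode.
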(event OnClicked(SM_Torch_Var01)
  (params (TouchedComponent :type Primitive%20Component%20Object%20Reference) (ButtonPressed :type Key%20Structure :default "None"))
  ;[1 1 1] Click events
  (if (Utilities|Enum|Equal(Enum) (Class|KismetInputLibrary|KeyGetDisplayName ButtonPressed) (Variables|Default|GetLMB))
    (Variables|Default|SetTorchClicked true)
    (Variables|/Script/Engine.PlayerController|SetbShowMouseCursor (Game|GetPlayerController 0) false)))

(event OnClicked(Sphere)
  (params (TouchedComponent :type Primitive%20Component%20Object%20Reference) (ButtonPressed :type Key%20Structure :default "None"))
  ;[1 1 1] Click events
  (if (Utilities|Enum|Equal(Enum) (Class|KismetInputLibrary|KeyGetDisplayName ButtonPressed) (Variables|Default|GetLMB))
    (Variables|Default|SetTorchClicked true)
    (Variables|/Script/Engine.PlayerController|SetbShowMouseCursor (Game|GetPlayerController 0) false)))

(event OnComponentBeginOverlap(Box)
  (params (OverlappedComponent :type Primitive%20Component%20Object%20Reference) (OtherActor :type Actor%20Object%20Reference) (OtherComp :type Primitive%20Component%20Object%20Reference) (OtherBodyIndex :type Integer) (bFromSweep :type Boolean) (SweepResult :type Hit%20Result%20Structure%20%28by%20ref%29))
  (bind _particlesystem (Variables|Default|GetParticleSystem))
  ;[1 1 1] On / off
  (if (== OtherActor (Game|GetPlayerCharacter 0))
    (Utilities|FlowControl|Sequence
      (:then_0
        (Utilities|FlowControl|Gate true) ; enters at Open
      )
      (:then_1
        (Utilities|FlowControl|Gate true) ; enters at Open
      ))))

(event OnComponentEndOverlap(Box)
  (params (OverlappedComponent :type Primitive%20Component%20Object%20Reference) (OtherActor :type Actor%20Object%20Reference) (OtherComp :type Primitive%20Component%20Object%20Reference) (OtherBodyIndex :type Integer))
  (bind _particlesystem (Variables|Default|GetParticleSystem))
  ;[1 1 1] On / off
  (if (== OtherActor (Game|GetPlayerCharacter 0))
    (Utilities|FlowControl|Sequence
      (:then_0
        (Utilities|FlowControl|Gate true) ; enters at Close
      )
      (:then_1
        (Utilities|FlowControl|Gate true) ; enters at Close
      ))))

(event OnComponentBeginOverlap(SM_Torch_Var01)
  (params (OverlappedComponent :type Primitive%20Component%20Object%20Reference) (OtherActor :type Actor%20Object%20Reference) (OtherComp :type Primitive%20Component%20Object%20Reference) (OtherBodyIndex :type Integer) (bFromSweep :type Boolean) (SweepResult :type Hit%20Result%20Structure%20%28by%20ref%29))
  ;[1 1 1] Spell Stages
  (Variables|Default|SetOverlapped (.LeftS (Utilities|String|Split (Utilities|String|RightChop (Utilities|GetDisplayName OtherComp) 17) " ")))
  (switch int (Variables|Default|GetStage)
    (:0
      (if (Utilities|Enum|Equal(Enum) (Variables|Default|GetOverlapped) (Variables|Default|GetNotch2String))
        (Components|Activation|Activate (Variables|Default|GetPos2) true)
        (Math|Integer|IncrementInt (Variables|Default|GetStage))))
    (:1
      (if (Utilities|Enum|Equal(Enum) (Variables|Default|GetOverlapped) (Variables|Default|GetNotch1String))
        (Components|Activation|Activate (Variables|Default|GetPos1) true)
        (Math|Integer|IncrementInt (Variables|Default|GetStage))))
    (:2
      (if (Utilities|Enum|Equal(Enum) (Variables|Default|GetOverlapped) (Variables|Default|GetNotch3String))
        (Components|Activation|Activate (Variables|Default|GetPos3) true)
        (Math|Integer|IncrementInt (Variables|Default|GetStage))))
    (:3
      (if (Utilities|Enum|Equal(Enum) (Variables|Default|GetOverlapped) (Variables|Default|GetNotch1String))
        (Components|Activation|Activate (Variables|Default|GetPos1) true)
        (Math|Integer|IncrementInt (Variables|Default|GetStage))))
    (:4
      (if (Utilities|Enum|Equal(Enum) (Variables|Default|GetOverlapped) (Variables|Default|GetNotch4String))
        (Utilities|Time|SetTimerbyFunctionName 0 "FinalStage" 3.0)))))

(event OnComponentEndOverlap(SM_Torch_Var01)
  (params (OverlappedComponent :type Primitive%20Component%20Object%20Reference) (OtherActor :type Actor%20Object%20Reference) (OtherComp :type Primitive%20Component%20Object%20Reference) (OtherBodyIndex :type Integer))
  ;[1 1 1] Spell Stages
  (Variables|Default|SetLeftOverlap (.LeftS (Utilities|String|Split (Utilities|String|RightChop (Utilities|GetDisplayName OtherComp) 17) " ")))
  (switch int (Variables|Default|GetStage)
    (:4
      (Utilities|Time|ClearTimerbyFunctionName 0 "FinalStage"))))

(event Custom|TurnOn
  (bind _returnvalue (Game|GetPlayerController 0))
  (bind _returnvalue_2 (Game|GetPlayerController 0))
  (bind _returnvalue_3 (Game|GetPlayerController 0))
  (bind _sm_torch_var01 (Variables|Default|GetSM_Torch_Var01))
  (bind _returnvalue_4 (Transformation|GetWorldLocation _sm_torch_var01))
  (bind _returnvalue_5 (+ _returnvalue_4 "0, 0,60.000000"))
  (bind _screenlocation (Class|PlayerController|ProjectWorldLocationtoScreen _returnvalue_3 _returnvalue_5 true))
  ;[1 1 1] Turn on
  (Input|DisableInput (Game|GetPlayerCharacter 0) _returnvalue)
  (Game|Player|SetViewTargetwithBlend _returnvalue self 0.5 "VTBlend_Linear" 0.0 false)
  (Utilities|FlowControl|Delay 0.5)
  (Variables|/Script/Engine.PlayerController|SetbShowMouseCursor _returnvalue_2 true)
  (Variables|/Script/Engine.PlayerController|SetbEnableClickEvents _returnvalue_2 true)
  (Actor|Tick|SetActorTickEnabled true)
  (Class|PlayerController|SetMouseLocation (Game|GetPlayerController 0) (Math|Float|Truncate (.x _screenlocation)) (Math|Float|Truncate (.y _screenlocation)))
  (CallFunction|StartSounds)
  (CallFunction|InitSpell)
  (Transformation|SetActorLocation (Game|GetPlayerCharacter 0) (Transformation|GetWorldLocation (Variables|Default|GetScene)) false false)
  (Pawn|SetControlRotation (Game|GetPlayerController 0) (.rotation (Transformation|GetWorldTransform (Variables|Default|GetCamera)))))

(event Custom|TurnOff
  (bind _returnvalue (Game|GetPlayerController 0))
  (bind _returnvalue_2 (Game|GetPlayerController 0))
  ;[1 1 1] TurnOff
  (Variables|/Script/Engine.PlayerController|SetbShowMouseCursor _returnvalue false)
  (Variables|/Script/Engine.PlayerController|SetbEnableClickEvents _returnvalue false)
  (Actor|Tick|SetActorTickEnabled false)
  (CallFunction|StopSounds)
  (Components|Activation|Deactivate (Variables|/Game/Audio/_BluePrints/BP_DC_MagicSliderSpell.BP_DC_MagicSliderSpell_C|GetParticleSystem (Variables|Default|GetParticleSystem)))
  (Input|EnableInput (Game|GetPlayerCharacter 0) _returnvalue_2)
  (Class|WidgetBlueprintLibrary|SetFocustoGameViewport)
  (Input|SetInputModeGameOnly _returnvalue_2)
  (Game|Player|SetViewTargetwithBlend (Game|GetPlayerController 0) (Game|GetPlayerCharacter 0) 0.5 "VTBlend_Linear" 0.0 false))

(event Custom|InitSpell
  (bind _curve (Variables|Default|GetCurve))
  (bind _curvetime (Variables|Default|GetCurveTime))
  (bind _returnvalue (Math|Curves|GetFloatValue _curve _curvetime))
  ;[1 1 1] Scale particle system
  (Transformation|SetActorScale3D (Variables|Default|GetParticleSystem) (Math|Vector|MakeVector _returnvalue _returnvalue _returnvalue))
  ;[1 1 1] Set Volumes
  (Audio|Components|Audio|SetVolumeMultiplier (Variables|Default|GetLayer_01_Audio) (Math|Curves|GetFloatValue (Variables|Default|GetLayer_01) (Variables|Default|GetCurveTime)) :!class /Script/Engine.AudioComponent)
  (Audio|Components|Audio|SetVolumeMultiplier (Variables|Default|GetLayer_02_Audio) (Math|Curves|GetFloatValue (Variables|Default|GetLayer_02) (Variables|Default|GetCurveTime)) :!class /Script/Engine.AudioComponent))

(event Custom|StopSounds
  (bind _layer_02_audio (Variables|Default|GetLayer_02_Audio))
  (bind _layer_01_audio (Variables|Default|GetLayer_01_Audio))
  ;[1 1 1] Stop sounds
  (Utilities|IsValid _layer_01_audio
    (:Is%20Valid
      (Audio|Components|Audio|FadeOut _layer_01_audio 1.0 0.0 :!class /Script/Engine.AudioComponent)
      (Utilities|IsValid _layer_02_audio
        (:Is%20Valid
          (Audio|Components|Audio|FadeOut _layer_02_audio 1.0 0.0 :!class /Script/Engine.AudioComponent))))))

(event Custom|StartSounds
  ;[1 1 1] Start Sounds
  (bind _returnvalue (Audio|SpawnSoundAttached "/Game/Audio/Magic/Stone_Circle_02_Magic_Spell_Layer_02.Stone_Circle_02_Magic_Spell_Layer_02" (Variables|/Script/Engine.Actor|GetRootComponent (Variables|Default|GetParticleSystem)) "None" "0, 0, 0" "0, 0, 0" "KeepRelativeOffset" false 1.0 1.0 0.0 0 0))
  (Variables|Default|SetLayer_01_Audio _returnvalue)
  (bind _returnvalue_2 (Audio|SpawnSoundAttached "/Game/Audio/Magic/Stone_Circle_02_Magic_Spell_Layer_01.Stone_Circle_02_Magic_Spell_Layer_01" (Variables|/Script/Engine.Actor|GetRootComponent (Variables|Default|GetParticleSystem)) "None" "0, 0, 0" "0, 0, 0" "KeepRelativeOffset" false 1.0 1.0 0.0 0 0))
  (Variables|Default|SetLayer_02_Audio _returnvalue_2))

(event Custom|FinalStage
  (bind _magicstone (Variables|Default|GetMagicStone))
  (bind _particlesystem (Variables|Default|GetParticleSystem))
  (bind _returnvalue (Transformation|GetActorLocation _particlesystem))
  ;[1 1 1] Spell Complete - Stone rising
  (Components|Activation|Activate (Variables|Default|GetPos4) true)
  (Math|Integer|IncrementInt (Variables|Default|GetStage)
    (:%20%20
      (Actor|Tick|SetActorTickEnabled false)
      (Variables|Default|SetMagicStoneStartLoc (Transformation|GetActorLocation (Variables|Default|GetMagicStone)))
      (Effects|SpawnEmitteratLocation "/Game/InfinityBladeEffects/Effects/FX_Monsters/FX_Monster_Elemental/ICE/P_Beam_Laser_Ice_BuildUP.P_Beam_Laser_Ice_BuildUP" _returnvalue "0, 0, 0" "3.000000,3.000000,3.000000")
      (Utilities|FlowControl|Sequence
        (:then_0
          (bind _newtrack_0 (Timeline|Timeline_0 PlayFromStart)
            (:Update
              (Transformation|SetActorScale3D (Variables|Default|GetParticleSystem) (Math|Vector|MakeVector _newtrack_0 _newtrack_0 _newtrack_0))
              (Audio|Components|Audio|SetVolumeMultiplier (Variables|Default|GetLayer_01_Audio) _newtrack_0 :!class /Script/Engine.AudioComponent)
              (Audio|Components|Audio|SetVolumeMultiplier (Variables|Default|GetLayer_02_Audio) _newtrack_0 :!class /Script/Engine.AudioComponent)
              (Transformation|SetActorLocation (Variables|Default|GetMagicStone) (Math|Vector|MakeVector (.x (Variables|Default|GetMagicStoneStartLoc)) (.y (Variables|Default|GetMagicStoneStartLoc)) (+ (.z (Variables|Default|GetMagicStoneStartLoc)) (* (- 1.0 _newtrack_0) 1.8e+02))) false false))
            (:Finished
              (Audio|Components|Audio|FadeOut (stale _returnvalue_2) 0.6 0.0 :!class /Script/Engine.AudioComponent)
              (Audio|PlaySoundatLocation "/Game/Audio/Props/Cave_Door_Stop.Cave_Door_Stop" _returnvalue "0, 0, 0" 0.4 1.0 0.0 0 0 0)
              (Utilities|FlowControl|Delay 1.0)
              (Default|Activate _magicstone)
              (Audio|PlaySoundatLocation "/Game/Audio/Magic/Magic_bolt_spell_stone_active.Magic_bolt_spell_stone_active" (Transformation|GetActorLocation _magicstone) "0, 0, 0" 1.0 1.0 0.0 "/Game/Audio/_Attenutations/Magic_Stone.Magic_Stone" 0 0)
              (Utilities|FlowControl|Delay 1.5)
              (CallFunction|TurnOff)
              (Timeline|Timeline_0 Stop))))
        (:then_1
          (bind _returnvalue_2 (Audio|SpawnSoundatLocation "/Game/Audio/Props/Cave_Door_Moving.Cave_Door_Moving" _returnvalue "0, 0, 0" 0.7 1.0 0.0 0 0)))))))

(event EventTick
  (params (DeltaSeconds :type Float%20%28single-precision%29))
  (bind _torchstartloc (Variables|Default|GetTorchStartLoc))
  (bind _torchstartloc_2 (Variables|Default|GetTorchStartLoc))
  (bind _sm_torch_var01 (Variables|Default|GetSM_Torch_Var01))
  (bind _torchstartloc_3 (Variables|Default|GetTorchStartLoc))
  (bind (_x _y _z) (Math|Vector|BreakVector _torchstartloc_3))
  (bind (_x_2 _y_2 _z_2) (Math|Vector|BreakVector _torchstartloc))
  (bind _relativelocation (Variables|/Script/Engine.SceneComponent|GetRelativeLocation _sm_torch_var01))
  (bind _relativelocation_2 (Variables|/Script/Engine.SceneComponent|GetRelativeLocation _sm_torch_var01))
  (bind _returnvalue (- _relativelocation_2 _torchstartloc_2))
  ;[1 1 1] Move torch
  (bind _returnvalue_2 (Class|WidgetLayoutLibrary|GetMousePositiononViewport))
  (Variables|Default|SetCurrentMouseX (.x _returnvalue_2))
  (Variables|Default|SetMouseDelta (- (Variables|Default|GetCurrentMouseX) (Variables|Default|GetPreviousMouseX)))
  (Variables|Default|SetPreviousMouseX (Variables|Default|GetCurrentMouseX))
  (if (Variables|Default|GetTorchClicked)
    (if (>= (.x _returnvalue) 0.0)
      (if (<= (.x _returnvalue) 2.4e+02)
        (Transformation|SetRelativeLocation (Variables|Default|GetSM_Torch_Var01) (Math|Vector|MakeVector (+ (* (Variables|Default|GetMouseDelta) (Variables|Default|GetSlideSpeed)) (.x _relativelocation)) (.y _relativelocation) (.z _relativelocation)) false false)
        (Variables|Default|SetPreviousMouseX (Variables|Default|GetCurrentMouseX))
        ;[1 1 1] Scale particle system
        (Variables|Default|SetCurveTime (Math|Float|MapRangeClamped (.x (- (Variables|/Script/Engine.SceneComponent|GetRelativeLocation (Variables|Default|GetSM_Torch_Var01)) (Variables|Default|GetTorchStartLoc))) 0.0 2.5e+02 0.0 1.0))
        (Transformation|SetActorScale3D (Variables|Default|GetParticleSystem) (Math|Vector|MakeVector (Math|Curves|GetFloatValue (Variables|Default|GetCurve) (Variables|Default|GetCurveTime)) (Math|Curves|GetFloatValue (Variables|Default|GetCurve) (Variables|Default|GetCurveTime)) (Math|Curves|GetFloatValue (Variables|Default|GetCurve) (Variables|Default|GetCurveTime))))
        ;[1 1 1] Set Volumes
        (Audio|Components|Audio|SetVolumeMultiplier (Variables|Default|GetLayer_01_Audio) (Math|Curves|GetFloatValue (Variables|Default|GetLayer_01) (Variables|Default|GetCurveTime)) :!class /Script/Engine.AudioComponent)
        (Audio|Components|Audio|SetVolumeMultiplier (Variables|Default|GetLayer_02_Audio) (Math|Curves|GetFloatValue (Variables|Default|GetLayer_02) (Variables|Default|GetCurveTime)) :!class /Script/Engine.AudioComponent)
        (else
          (Transformation|SetRelativeLocation (Variables|Default|GetSM_Torch_Var01) (Math|Vector|MakeVector (+ _x_2 239.0) _y_2 _z_2) false false)))
      (else
        (Transformation|SetRelativeLocation (Variables|Default|GetSM_Torch_Var01) (Math|Vector|MakeVector (+ _x 1.0) _y _z) false false)))))

(event EventBeginPlay
  ;[1 1 1] Get torch start location
  (Variables|Default|SetTorchStartLoc (Variables|/Script/Engine.SceneComponent|GetRelativeLocation (Variables|Default|GetSM_Torch_Var01))))

(event Input|MouseEvents|LeftMouseButton
  (params (Key :type Key%20Structure :default "None"))
  ;[1 1 1] On / off
  (:Released
    (Utilities|FlowControl|Gate true
      (:Exit
        (Variables|Default|SetTorchClicked false)
        (Variables|/Script/Engine.PlayerController|SetbShowMouseCursor (Game|GetPlayerController 0) true)))))

(event Input|KeyboardEvents|E
  (params (Key :type Key%20Structure :default "None"))
  (bind _particlesystem (Variables|Default|GetParticleSystem))
  ;[1 1 1] On / off
  (:Pressed
    (Utilities|FlowControl|Gate true
      (:Exit
        (if (Variables|Default|GetUnlocked)
          (Utilities|FlowControl|FlipFlop
            (:A
              (CallFunction|Turnon)
              (Default|Turnon _particlesystem))
            (:B
              (CallFunction|TurnOff)
              (Default|TurnOff _particlesystem)
              (Variables|Default|SetTorchClicked false))))))))

(fn ConstructionScript)