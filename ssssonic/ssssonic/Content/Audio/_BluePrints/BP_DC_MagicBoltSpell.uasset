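; Magic bolt spell actor that lets the player, while inside its sphere, charge and fire a BP_DC_MagicBolt with the left mouse button.
; Charging follows the player's spell socket, growing the FX on Tick while a timeline drives two layered sound volumes.
; Release spawns the bolt, deriving its size, power and fire volume from the charge scale.
; It also plays fairy dialogue on first overlap and as stones are activated.
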(event OnComponentBeginOverlap(Sphere)
  (params (OverlappedComponent :type Primitive%20Component%20Object%20Reference) (OtherActor :type Actor%20Object%20Reference) (OtherComp :type Primitive%20Component%20Object%20Reference) (OtherBodyIndex :type Integer) (bFromSweep :type Boolean) (SweepResult :type Hit%20Result%20Structure%20%28by%20ref%29))
  ;[1 1 1] Input and Dialogue
  (if (== OtherActor (Game|GetPlayerCharacter 0))
    (Utilities|FlowControl|Sequence
      (:then_0
        (Utilities|FlowControl|Sequence
          (:then_0
            (Utilities|FlowControl|Gate true) ; enters at Open
          )
          (:then_1
            (Utilities|FlowControl|Gate true) ; enters at Open
          )))
      (:then_1
        (Utilities|FlowControl|DoOnce false
          (:Completed
            (Audio|SpawnSoundatLocation "/Game/Audio/Dialogue/Fairy_03/Fairy_03_Spell.Fairy_03_Spell" (Transformation|GetActorLocation self) "0, 0, 0" 1.0 1.0 0.0 0 0)))))))

(event OnComponentEndOverlap(Sphere)
  (params (OverlappedComponent :type Primitive%20Component%20Object%20Reference) (OtherActor :type Actor%20Object%20Reference) (OtherComp :type Primitive%20Component%20Object%20Reference) (OtherBodyIndex :type Integer))
  ;[1 1 1] Input and Dialogue
  (if (== OtherActor (Game|GetPlayerCharacter 0))
    (Utilities|FlowControl|Sequence
      (:then_0
        (Utilities|FlowControl|Gate true) ; enters at Close
      )
      (:then_1
        (Utilities|FlowControl|Gate true) ; enters at Close
      ))))

(event Custom|ChargeSpell
  (bind _self self)
  (bind _rootcomponent (Variables|Transformation|GetRootComponent _self))
  ;[1 1 1] Start charging
  (Transformation|SetWorldScale3D (Variables|Default|GetChargingFX) (Variables|Default|GetInitialScale))
  (Actor|Tick|SetActorTickEnabled true)
  (Components|Activation|Activate (Variables|Default|GetChargingFX) false)
  (Variables|Default|SetCharging true)
  ;[1 1 1] spawn sounds and set volumes
  (bind _returnvalue (Audio|SpawnSoundAttached "/Game/Audio/Magic/Magic_Bolt_Layer_01.Magic_Bolt_Layer_01" _rootcomponent "None" "0, 0, 0" "0, 0, 0" "KeepRelativeOffset" false 1.2 1.0 0.0 0 0))
  (bind _returnvalue_2 (Audio|SpawnSoundAttached "/Game/Audio/Magic/Magic_Bolt_Layer_02.Magic_Bolt_Layer_02" _rootcomponent "None" "0, 0, 0" "0, 0, 0" "KeepRelativeOffset" false 1.2 1.0 0.0 0 0))
  (bind (_direction _newtrack_0 _newtrack_3) (Timeline|Bolt_Loop_Volume PlayFromStart)
    (:Update
      (Audio|Components|Audio|SetVolumeMultiplier _returnvalue _newtrack_0 :!class /Script/Engine.AudioComponent)
      (Audio|Components|Audio|SetVolumeMultiplier _returnvalue_2 _newtrack_3 :!class /Script/Engine.AudioComponent))))

(event Custom|ReleaseSpell
  (bind _chargingfx (Variables|Default|GetChargingFX))
  (bind _chargescalingfactor (Variables|Default|GetChargeScalingFactor))
  (bind _returnvalue (Transformation|GetWorldScale _chargingfx))
  (bind _returnvalue_2 (* _returnvalue _chargescalingfactor))
  (bind _returnvalue_3 (Math|Vector|ClampVectorSize _returnvalue_2 0.0 0.7))
  (bind _x (Math|Vector|BreakVector _returnvalue_3))
  ;[1 1 1] Release spell
  (Components|Activation|Deactivate (Variables|Default|GetChargingFX))
  (Variables|Default|SetCharging false)
  (bind _asfirst_person_character (Utilities|Casting|CastToFirstPersonCharacter (Game|GetPlayerCharacter 0)))
  (Variables|Default|SetLaunchLocation (+ (Transformation|GetWorldLocation (Variables|/Game/FirstPersonBP/Blueprints/FirstPersonCharacter.FirstPersonCharacter_C|GetSpellSocket _asfirst_person_character)) (Variables|Default|GetLaunchOffset)))
  (bind _returnvalue_4 (Game|SpawnActorfromClass "/Game/Audio/_BluePrints/BP_DC_MagicBolt.BP_DC_MagicBolt_C" (Math|Transform|MakeTransform (Variables|Default|GetLaunchLocation) (Math|Rotator|MakeRotator (+ (.roll (Transformation|GetWorldRotation (Variables|/Game/FirstPersonBP/Blueprints/FirstPersonCharacter.FirstPersonCharacter_C|GetFirstPersonCamera _asfirst_person_character))) 0.0) (+ (.pitch (Transformation|GetWorldRotation (Variables|/Game/FirstPersonBP/Blueprints/FirstPersonCharacter.FirstPersonCharacter_C|GetFirstPersonCamera _asfirst_person_character))) 1.0) (+ (.yaw (Transformation|GetWorldRotation (Variables|/Game/FirstPersonBP/Blueprints/FirstPersonCharacter.FirstPersonCharacter_C|GetFirstPersonCamera _asfirst_person_character))) -3.0)) (* (Transformation|GetWorldScale (Variables|Default|GetChargingFX)) (Variables|Default|GetBoltScalingFactor))) "Undefined" 0 0))
  (Variables|/Game/Audio/_BluePrints/BP_DC_MagicBolt.BP_DC_MagicBolt_C|SetPower _returnvalue_4 _x)
  (Audio|SpawnSoundAttached "/Game/Audio/Magic/Magic_bolt_spell_fire.Magic_bolt_spell_fire" (Variables|Transformation|GetRootComponent self) "None" "0, 0, 0" "0, 0, 0" "KeepRelativeOffset" false (Math|Float|MapRangeClamped _x 0.05 0.41 0.1 1.2) 1.0 0.0 0 0)
  ;[1 1 1] spawn sounds and set volumes
  (Audio|Components|Audio|FadeOut (stale Custom|ChargeSpell _returnvalue) 0.001 0.0 :!class /Script/Engine.AudioComponent) ; ???
  (bind (_direction _newtrack_0 _newtrack_3) (Timeline|Bolt_Loop_Volume Stop)
    (:Update
      (Audio|Components|Audio|SetVolumeMultiplier (stale Custom|ChargeSpell _returnvalue) _newtrack_0 :!class /Script/Engine.AudioComponent)
      (Audio|Components|Audio|SetVolumeMultiplier (stale Custom|ChargeSpell _returnvalue_2) _newtrack_3 :!class /Script/Engine.AudioComponent))))

(event Custom|Increment_Stones
  (bind _self self)
  (bind _returnvalue (Transformation|GetActorLocation _self))
  ;[1 1 1] Input and Dialogue
  (Utilities|FlowControl|DoOnce false
    (:Completed
      (switch int (Variables|Default|GetStones_Activated)
        (:0
          (Audio|SpawnSoundatLocation "/Game/Audio/Dialogue/Fairy_03/Fairy_03_First_Stone.Fairy_03_First_Stone" _returnvalue "0, 0, 0" 1.0 1.0 0.0 0 0)
          (Math|Integer|IncrementInt (Variables|Default|GetStones_Activated) :!label _label
            (:%20%20
              (CallFunction|Reset))))
        (:1
          (Audio|SpawnSoundatLocation "/Game/Audio/Dialogue/Fairy_03/Fairy_03_Second_Stone.Fairy_03_Second_Stone" _returnvalue "0, 0, 0" 1.0 1.0 0.0 0 0)
          (goto _label))
        (:2
          (Audio|SpawnSoundatLocation "/Game/Audio/Dialogue/Fairy_03/Fairy_03_Third_Stone_Complete.Fairy_03_Third_Stone_Complete" _returnvalue "0, 0, 0" 1.0 1.0 0.0 0 0))))))

(event Custom|Reset
  (bind _self self)
  (bind _returnvalue (Transformation|GetActorLocation _self))
  ;[1 1 1] Input and Dialogue
  (Utilities|FlowControl|DoOnce false) ; enters at Reset
)

(event EventTick
  (params (DeltaSeconds :type Float%20%28single-precision%29))
  ;[1 1 1] Charge spell
  (if (Variables|Default|GetCharging)
    (bind _asfirst_person_character (Utilities|Casting|CastToFirstPersonCharacter (Game|GetPlayerCharacter 0)))
    (Transformation|SetActorRotation (Transformation|GetWorldRotation (Variables|/Game/FirstPersonBP/Blueprints/FirstPersonCharacter.FirstPersonCharacter_C|GetFirstPersonCamera _asfirst_person_character)))
    (Transformation|SetActorLocation (+ (Transformation|GetWorldLocation (Variables|/Game/FirstPersonBP/Blueprints/FirstPersonCharacter.FirstPersonCharacter_C|GetSpellSocket _asfirst_person_character)) (Math|Vector|MakeVector 0.0 0.0 (Variables|Default|GetHeightOffsetCharge))) false false)
    (Transformation|SetWorldScale3D (Variables|Default|GetChargingFX) (Math|Vector|ClampVectorSize (* (Transformation|GetWorldScale (Variables|Default|GetChargingFX)) (Variables|Default|GetChargeScalingFactor)) 0.0 0.7))))

(event EventBeginPlay
  ;[1 1 1] Get starting scale
  (Variables|Default|SetInitialScale (Transformation|GetWorldScale (Variables|Default|GetChargingFX))))

(event Input|MouseEvents|LeftMouseButton
  (params (Key :type Key%20Structure :default "None"))
  ;[1 1 1] Input and Dialogue
  (:Pressed
    (Utilities|FlowControl|Gate true
      (:Exit
        (Components|Activation|Activate (Variables|Default|GetChargingFX) false)
        (CallFunction|ChargeSpell))))
  (:Released
    (Utilities|FlowControl|Gate true
      (:Exit
        (CallFunction|ReleaseSpell)))))

(event Input|KeyboardEvents|R
  (params (Key :type Key%20Structure :default "None"))
  (bind _bolt_loop_volume (Variables|Default|GetBolt_Loop_Volume))
  ;[1 1 1] change play rate
  (:Pressed
    (Utilities|FlowControl|FlipFlop
      (:A
        (Components|Timeline|SetPlayRate _bolt_loop_volume 1.0))
      (:B
        (Components|Timeline|SetPlayRate _bolt_loop_volume 4.0)))))

(fn ConstructionScript)