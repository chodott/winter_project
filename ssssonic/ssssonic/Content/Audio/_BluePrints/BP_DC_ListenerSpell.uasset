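; Trigger-volume actor for a "listener spell" that lets the player move the audio listener to a clicked point in the world.
; While the player is inside the box, E enables the cursor and click mode through a FlipFlop whose off branch is empty.
; A click traces to the hit, moves the listener there and shows a HUD camera view placed short of it.
; Leaving the box restores game input and the player-camera listener.
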(event OnComponentBeginOverlap(Box)
  (params (OverlappedComponent :type Primitive%20Component%20Object%20Reference) (OtherActor :type Actor%20Object%20Reference) (OtherComp :type Primitive%20Component%20Object%20Reference) (OtherBodyIndex :type Integer) (bFromSweep :type Boolean) (SweepResult :type Hit%20Result%20Structure%20%28by%20ref%29))
  (bind _returnvalue (Game|GetPlayerController 0))
  (bind _returnvalue_2 (Game|GetPlayerController 0))
  (bind (_sizex _sizey) (HUD|GetViewportSize _returnvalue_2))
  ;[1 1 1] toggle listener spell on/off
  (if (== OtherActor (Game|GetPlayerCharacter 0))
    (Utilities|FlowControl|Gate true) ; enters at Open
  ))

(event OnComponentEndOverlap(Box)
  (params (OverlappedComponent :type Primitive%20Component%20Object%20Reference) (OtherActor :type Actor%20Object%20Reference) (OtherComp :type Primitive%20Component%20Object%20Reference) (OtherBodyIndex :type Integer))
  (bind _returnvalue (Game|GetPlayerController 0))
  (bind _returnvalue_2 (Game|GetPlayerController 0))
  (bind _returnvalue_3 (Game|GetPlayerController 0))
  (bind _returnvalue_4 (Game|GetPlayerController 0))
  (bind (_sizex _sizey) (HUD|GetViewportSize _returnvalue_4))
  ;[1 1 1] toggle listener spell on/off
  (if (== OtherActor (Game|GetPlayerCharacter 0))
    (Utilities|FlowControl|Sequence
      (:then_0
        (Utilities|FlowControl|Gate true) ; enters at Close
      )
      (:then_1
        (Variables|/Script/Engine.PlayerController|SetbShowMouseCursor _returnvalue_2 false)
        (Variables|/Script/Engine.PlayerController|SetbEnableClickEvents _returnvalue_2 false)
        (Variables|Default|SetActive false)
        (bind _asfirst_person_hud (Utilities|Casting|CastToFirstPersonHUD (HUD|GetHUD _returnvalue)))
        (Variables|/Game/FirstPersonBP/Blueprints/FirstPersonHUD.FirstPersonHUD_C|SetDrawListenerCamera _asfirst_person_hud false)
        (Input|SetInputModeGameOnly _returnvalue)
        (Class|WidgetBlueprintLibrary|SetFocustoGameViewport)
        (bind _asfirst_person_character (Utilities|Casting|CastToFirstPersonCharacter (Game|GetPlayerCharacter 0)))
        (Class|PlayerController|SetAudioListenerOverride (Game|GetPlayerController 0) (Variables|/Game/FirstPersonBP/Blueprints/FirstPersonCharacter.FirstPersonCharacter_C|GetFreecamera _asfirst_person_character) "0, 0, 0" "0, 0, 0")))))

(event Input|MouseEvents|LeftMouseButton
  (params (Key :type Key%20Structure :default "None"))
  (bind _returnvalue (Game|GetPlayerController 0))
  (bind (_worldlocation _worlddirection) (Game|Player|ConvertMouseLocationToWorldSpace _returnvalue))
  ;[1 1 1] set position of listener
  (:Pressed
    (if (Variables|Default|GetActive)
      (Variables|Default|SetMouseLocation _worldlocation)
      (Variables|Default|SetMouseDirection _worlddirection)
      (bind _outhit (Collision|LineTraceByChannel (Variables|Default|GetMouseLocation) (+ (Variables|Default|GetMouseLocation) (* (Variables|Default|GetMouseDirection) 5e+04)) "TraceTypeQuery1" false 0 "None"))
      (Variables|Default|SetHitLocation (.Location (Collision|BreakHitResult _outhit)))
      (Class|PlayerController|SetAudioListenerOverride (Game|GetPlayerController 0) 0 (Variables|Default|GetHitLocation) "0, 0, 0")
      (bind _asfirst_person_character (Utilities|Casting|CastToFirstPersonCharacter (Game|GetPlayerCharacter 0)))
      (Transformation|SetActorTransform (Variables|Default|GetListenerCamera) (Math|Transform|MakeTransform (+ (Transformation|GetWorldLocation (Variables|/Game/FirstPersonBP/Blueprints/FirstPersonCharacter.FirstPersonCharacter_C|GetFreecamera _asfirst_person_character)) (* (Math|Vector|GetForwardVector (Math|Rotator|FindLookatRotation (Transformation|GetWorldLocation (Variables|/Game/FirstPersonBP/Blueprints/FirstPersonCharacter.FirstPersonCharacter_C|GetFreecamera _asfirst_person_character)) (Variables|Default|GetHitLocation))) (- (Math|Vector|Distance(Vector) (Transformation|GetWorldLocation (Variables|/Game/FirstPersonBP/Blueprints/FirstPersonCharacter.FirstPersonCharacter_C|GetFreecamera _asfirst_person_character)) (Variables|Default|GetHitLocation)) 4e+02))) (Math|Rotator|FindLookatRotation (Transformation|GetWorldLocation (Variables|/Game/FirstPersonBP/Blueprints/FirstPersonCharacter.FirstPersonCharacter_C|GetFreecamera _asfirst_person_character)) (Variables|Default|GetHitLocation)) "1,1,1"))
      (bind _asfirst_person_hud (Utilities|Casting|CastToFirstPersonHUD (HUD|GetHUD (Game|GetPlayerController 0))))
      (Variables|/Game/FirstPersonBP/Blueprints/FirstPersonHUD.FirstPersonHUD_C|SetDrawListenerCamera _asfirst_person_hud true))))

(event Input|KeyboardEvents|E
  (params (Key :type Key%20Structure :default "None"))
  (bind _returnvalue (Game|GetPlayerController 0))
  (bind _returnvalue_2 (Game|GetPlayerController 0))
  (bind (_sizex _sizey) (HUD|GetViewportSize _returnvalue_2))
  ;[1 1 1] toggle listener spell on/off
  (:Pressed
    (Utilities|FlowControl|Gate true
      (:Exit
        (Utilities|FlowControl|FlipFlop
          (:A
            (Input|SetInputModeGameandUI _returnvalue 0 "DoNotLock" true)
            (Variables|/Script/Engine.PlayerController|SetbShowMouseCursor _returnvalue true)
            (Variables|/Script/Engine.PlayerController|SetbEnableClickEvents _returnvalue true)
            (Variables|Default|SetActive true)
            (Class|PlayerController|SetMouseLocation _returnvalue_2 (/ _sizex 2) (/ _sizey 2))))))))

(fn ConstructionScript)