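; Interactive platform where the player spawns a rolling physics barrel and pushes it with a charged spell.
; Gates enable input only while the player is inside the trigger box.
; E breaks any existing barrel with particles and spawns a replacement after a short delay.
; Holding left mouse charges a physics spell; releasing it briefly fires the barrel's thruster, aligned to player yaw, with strength scaled by hold time.
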(event OnComponentBeginOverlap(TriggerBox)
  (params (OverlappedComponent :type Primitive%20Component%20Object%20Reference) (OtherActor :type Actor%20Object%20Reference) (OtherComp :type Primitive%20Component%20Object%20Reference) (OtherBodyIndex :type Integer) (bFromSweep :type Boolean) (SweepResult :type Hit%20Result%20Structure%20%28by%20ref%29))
  ;[1 1 1] Spawn barrel
  (if (== OtherActor (Game|GetPlayerCharacter 0))
    (Utilities|FlowControl|Sequence
      (:then_0
        (Utilities|FlowControl|Gate true) ; enters at Open
      )
      (:then_1
        ;[1 1 1] Charge spell & release
        (Utilities|FlowControl|Gate true) ; enters at Open
      )
      (:then_2
        (Utilities|FlowControl|Gate true) ; enters at Open
      ))))

(event OnComponentEndOverlap(TriggerBox)
  (params (OverlappedComponent :type Primitive%20Component%20Object%20Reference) (OtherActor :type Actor%20Object%20Reference) (OtherComp :type Primitive%20Component%20Object%20Reference) (OtherBodyIndex :type Integer))
  ;[1 1 1] Spawn barrel
  (if (== OtherActor (Game|GetPlayerCharacter 0))
    (Utilities|FlowControl|Sequence
      (:then_0
        (Utilities|FlowControl|Gate true) ; enters at Close
      )
      (:then_1
        ;[1 1 1] Charge spell & release
        (Utilities|FlowControl|Gate true) ; enters at Close
      )
      (:then_2
        (Utilities|FlowControl|Gate true) ; enters at Close
      ))))

(event Input|MouseEvents|LeftMouseButton
  (params (Key :type Key%20Structure :default "None"))
  (bind _barreltopush (Variables|Default|GetBarrelToPush))
  (bind _barreltopush_2 (Variables|Default|GetBarrelToPush))
  (bind _physicsthruster (Variables|/Game/Audio/_BluePrints/BP_DC_PhysicsBarrel_Rolling.BP_DC_PhysicsBarrel_Rolling_C|GetPhysicsThruster _barreltopush))
  ;[1 1 1] Charge spell & release
  (:Pressed
    (Utilities|FlowControl|Gate true
      (:Exit
        (Utilities|IsValid _barreltopush_2
          (:Is%20Valid
            (Variables|Default|SetMouseDownTime (Utilities|Time|GetTimeSeconds))
            (bind _returnvalue (Game|SpawnActorfromClass "/Game/Audio/_BluePrints/BP_DC_PhysicsSpell.BP_DC_PhysicsSpell_C" (Transformation|GetActorTransform) "Undefined" 0 0))
            (Variables|Default|SetPhysicsSpell _returnvalue)
            (Default|ChargeSpell (Variables|Default|GetPhysicsSpell)))))))
  (:Released
    (Utilities|FlowControl|Gate true
      (:Exit
        (Utilities|IsValid _barreltopush_2
          (:Is%20Valid
            (Transformation|SetWorldRotation _physicsthruster (Math|Rotator|MakeRotator 0.0 0.0 (- (.yaw (Transformation|GetActorRotation (Game|GetPlayerCharacter 0))) 1.8e+02)) false false)
            (Variables|/Script/Engine.PhysicsThrusterComponent|SetThrustStrength _physicsthruster (Math|Float|MapRangeClamped (- (Utilities|Time|GetTimeSeconds) (Variables|Default|GetMouseDownTime)) 0.0 2.0 1e+02 3e+05))
            (Components|Activation|Activate _physicsthruster true)
            (Default|ReleaseSpell (Variables|Default|GetPhysicsSpell))
            (Utilities|FlowControl|Delay 0.5)
            (Components|Activation|Deactivate (Variables|/Game/Audio/_BluePrints/BP_DC_PhysicsBarrel_Rolling.BP_DC_PhysicsBarrel_Rolling_C|GetPhysicsThruster (Variables|Default|GetBarrelToPush)))))))))

(event Input|KeyboardEvents|E
  (params (Key :type Key%20Structure :default "None"))
  ;[1 1 1] Spawn barrel
  (:Pressed
    (Utilities|FlowControl|Gate true
      (:Exit
        (if (Utilities|IsValid (Variables|Default|GetBarrelToPush))
          (Effects|SpawnEmitteratLocation "/Game/InfinityBladeEffects/Effects/FX_Breakables/barrel/P_BarrelBreak_Wood.P_BarrelBreak_Wood" (Transformation|GetWorldLocation (Variables|/Game/Audio/_BluePrints/BP_DC_PhysicsBarrel_Rolling.BP_DC_PhysicsBarrel_Rolling_C|GetStaticMesh (Variables|Default|GetBarrelToPush))) "0, 0, 0" "2.000000,2.000000,2.000000")
          (Actor|DestroyActor (Variables|Default|GetBarrelToPush)))
        (Components|Activation|Activate (Variables|Default|GetP_Summon_Child_Startup) false)
        (Utilities|FlowControl|Delay 0.5)
        (bind _returnvalue (Game|SpawnActorfromClass "/Game/Audio/_BluePrints/BP_DC_PhysicsBarrel_Rolling.BP_DC_PhysicsBarrel_Rolling_C" (Transformation|GetWorldTransform (Variables|Default|GetSpawnPoint)) "Undefined" 0 0))
        (Variables|Default|SetBarrelToPush _returnvalue)))))

(fn ConstructionScript)