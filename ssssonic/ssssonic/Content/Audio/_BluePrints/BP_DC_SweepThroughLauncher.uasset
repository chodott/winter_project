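; Audio launcher that repeatedly spawns sweep-through sound actors around the player character at random intervals.
; Start_Sweeper_Lp sets a randomized timer for Spawn_Sweeper, which re-arms it after each spawn; Stop_Sweeper_Lp clears it.
; Each BP_DC_SweepThrough_Sound spawns at a random offset along the player's forward, right and up axes, with a look-at rotation targeting the player.
; The launcher then passes its sound, attenuation and speed to the spawned actor.
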(event Custom|Spawn_Sweeper
  (bind _returnvalue (Game|GetPlayerCharacter 0))
  (bind _max (Variables|Default|GetMax))
  (bind _min (Variables|Default|GetMin))
  (bind _returnvalue_2 (Transformation|GetActorUpVector _returnvalue))
  (bind (_x _y _z) (Math|Vector|BreakVector _min))
  (bind (_x_2 _y_2 _z_2) (Math|Vector|BreakVector _max))
  (bind _returnvalue_3 (Transformation|GetActorLocation _returnvalue))
  (bind _returnvalue_4 (Transformation|GetActorForwardVector _returnvalue))
  (bind _returnvalue_5 (Transformation|GetActorRightVector _returnvalue))
  (bind _returnvalue_6 (Math|Random|RandomFloatinRange _z _z_2))
  (bind _returnvalue_7 (Math|Random|RandomFloatinRange _x _x_2))
  (bind _returnvalue_8 (Math|Random|RandomFloatinRange _y _y_2))
  (bind _returnvalue_9 (* _returnvalue_2 _returnvalue_6))
  (bind _returnvalue_10 (* _returnvalue_4 _returnvalue_7))
  (bind _returnvalue_11 (* _returnvalue_5 _returnvalue_8))
  (bind _returnvalue_12 (+ _returnvalue_10 _returnvalue_11 _returnvalue_9))
  (bind _returnvalue_13 (+ _returnvalue_3 _returnvalue_12))
  ;[1 1 1] Spawn Sweep Through Blueprint
  (bind _returnvalue_14 (Game|SpawnActorfromClass "/Game/Audio/_BluePrints/BP_DC_SweepThrough_Sound.BP_DC_SweepThrough_Sound_C" (Math|Transform|MakeTransform _returnvalue_13 (Math|Rotator|FindLookatRotation _returnvalue_13 (Transformation|GetActorLocation (Game|GetPlayerCharacter 0))) "1,1,1") "Undefined" 0 0))
  (Variables|/Game/Audio/_BluePrints/BP_DC_SweepThrough_Sound.BP_DC_SweepThrough_Sound_C|SetSound _returnvalue_14 (Variables|Default|GetSound))
  (Variables|/Game/Audio/_BluePrints/BP_DC_SweepThrough_Sound.BP_DC_SweepThrough_Sound_C|SetAttenuation _returnvalue_14 (Variables|Default|GetAttenuationSettings))
  (Variables|/Game/Audio/_BluePrints/BP_DC_SweepThrough_Sound.BP_DC_SweepThrough_Sound_C|SetSpeed _returnvalue_14 (Variables|Default|GetSpeed))
  ;[1 1 1] Timer
  (bind _returnvalue_15 (Utilities|Time|SetTimerbyFunctionName 0 "Spawn_Sweeper" (Math|Random|RandomFloatinRange (Variables|Default|GetMin_Spawn_Time) (Variables|Default|GetMax_Spawn_Time)))))

(event Custom|Start_Sweeper_Lp
  ;[1 1 1] Timer
  (bind _returnvalue (Utilities|Time|SetTimerbyFunctionName 0 "Spawn_Sweeper" (Math|Random|RandomFloatinRange (Variables|Default|GetMin_Spawn_Time) (Variables|Default|GetMax_Spawn_Time)))))

(event Custom|Stop_Sweeper_Lp
  ;[1 1 1] Timer
  (Utilities|Time|ClearandInvalidateTimerbyHandle (stale Custom|Spawn_Sweeper _returnvalue_15)))

(fn ConstructionScript)