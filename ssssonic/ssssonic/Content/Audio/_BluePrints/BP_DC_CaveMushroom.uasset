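; Cave mushroom actor with audio that the player can remove by pressing E while inside its sphere trigger.
; Sphere overlaps with the player character open and close a gate between the key press and DestroyActor.
; A ToggleListenerFocus event alternates the audio between focus-on and focus-off attenuation settings.
; A leftover Tick debug computes the player's facing angle to the mushroom, with screen and log output disabled.
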(event OnComponentBeginOverlap(Sphere)
  (params (OverlappedComponent :type Primitive%20Component%20Object%20Reference) (OtherActor :type Actor%20Object%20Reference) (OtherComp :type Primitive%20Component%20Object%20Reference) (OtherBodyIndex :type Integer) (bFromSweep :type Boolean) (SweepResult :type Hit%20Result%20Structure%20%28by%20ref%29))
  ;[1 1 1] Key press
  (if (== OtherActor (Game|GetPlayerCharacter 0))
    (Utilities|FlowControl|Gate true) ; enters at Open
  ))

(event OnComponentEndOverlap(Sphere)
  (params (OverlappedComponent :type Primitive%20Component%20Object%20Reference) (OtherActor :type Actor%20Object%20Reference) (OtherComp :type Primitive%20Component%20Object%20Reference) (OtherBodyIndex :type Integer))
  ;[1 1 1] Key press
  (if (== OtherActor (Game|GetPlayerCharacter 0))
    (Utilities|FlowControl|Gate true) ; enters at Close
  ))

(event Custom|ToggleListenerFocus
  ;[1 1 1] Toggle listener focus
  (Utilities|FlowControl|FlipFlop
    (:A
      (Audio|Components|Audio|AdjustAttenuation (Variables|Default|GetAudio) (Variables|/Script/Engine.SoundAttenuation|GetAttenuation (Variables|Default|GetFocusOn)))
      (Development|PrintString "Listener Focus On" false))
    (:B
      (Audio|Components|Audio|AdjustAttenuation (Variables|Default|GetAudio) (Variables|/Script/Engine.SoundAttenuation|GetAttenuation (Variables|Default|GetFocusOff)))
      (Development|PrintString "Listener Focus Off" false))))

(event EventTick
  (params (DeltaSeconds :type Float%20%28single-precision%29))
  (bind _returnvalue (Game|GetPlayerCharacter 0))
  ;[1 1 1] Debug
  (Development|PrintString (Utilities|String|ToString(Float) (Class|KismetMathLibrary|DegAcos (Math|Vector|DotProduct (Transformation|GetActorForwardVector _returnvalue) (Math|Vector|GetForwardVector (Math|Rotator|FindLookatRotation (Transformation|GetActorLocation _returnvalue) (Transformation|GetActorLocation self)))))) false false "(R=0.000000,G=0.660000,B=1.000000,A=1.000000)" DeltaSeconds))

(event Input|KeyboardEvents|E
  (params (Key :type Key%20Structure :default "None"))
  ;[1 1 1] Key press
  (:Pressed
    (Utilities|FlowControl|Gate true
      (:Exit
        (Actor|DestroyActor)))))

(fn ConstructionScript)