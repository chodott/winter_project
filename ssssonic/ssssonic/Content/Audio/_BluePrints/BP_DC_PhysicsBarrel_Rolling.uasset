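; Physics barrel Blueprint that plays impact and rolling sounds driven by its motion.
; Each Hit event compares impulse against a threshold for a one-shot, volume-scaled impact, and X-axis angular velocity against another for rolling.
; DoOnce gates prevent retriggering; rolling audio starts at a random offset, with volume and pitch following spin speed.
; Rolling fades out and resets when spin drops during a hit or on ActorEndOverlap.
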(event Collision|EventActorEndOverlap
  (params (OtherActor :type Actor%20Object%20Reference))
  (bind _rollingsound (Variables|Default|GetRollingSound))
  (bind _sound (Variables|/Script/Engine.AudioComponent|GetSound _rollingsound))
  (bind _duration (Variables|/Script/Engine.SoundBase|GetDuration _sound))
  (bind _returnvalue (- _duration 1.0))
  (bind _returnvalue_2 (Math|Random|RandomFloatinRange 0.0 _returnvalue))
  ;[1 1 1] play rolling sound
  (Audio|Components|Audio|FadeOut (Variables|Default|GetRollingSound) 0.1 0.0 :!class /Script/Engine.AudioComponent)
  (Utilities|FlowControl|DoOnce false) ; enters at Reset
)

(event Collision|EventHit
  (params (MyComp :type Primitive%20Component%20Object%20Reference) (Other :type Actor%20Object%20Reference) (OtherComp :type Primitive%20Component%20Object%20Reference) (bSelfMoved :type Boolean) (HitLocation :type Vector :default "0, 0, 0") (HitNormal :type Vector :default "0, 0, 0") (NormalImpulse :type Vector :default "0, 0, 0") (Hit :type Hit%20Result%20Structure%20%28by%20ref%29))
  (bind _rollingsound (Variables|Default|GetRollingSound))
  (bind _rollingsound_2 (Variables|Default|GetRollingSound))
  (bind _sound (Variables|/Script/Engine.AudioComponent|GetSound _rollingsound))
  (bind _duration (Variables|/Script/Engine.SoundBase|GetDuration _sound))
  (bind _returnvalue (- _duration 1.0))
  (bind _returnvalue_2 (Math|Random|RandomFloatinRange 0.0 _returnvalue))
  ;[1 1 1] Hit event - get speed
  (Variables|Default|SetForce (Math|Vector|VectorLength NormalImpulse))
  (Variables|Default|SetRotationSpeed (Math|Float|Absolute(Float) (.X (Math|Vector|BreakVector (Physics|GetPhysicsAngularVelocityinDegrees (Variables|Default|GetStaticMesh) "None")))))
  (Utilities|FlowControl|Sequence
    (:then_0
      ;[1 1 1] Threshold for impacts
      (if (> (Variables|Default|GetForce) 3e+03)
        ;[1 1 1] play impact sound
        (Utilities|FlowControl|DoOnce false :!label _label
          (:Completed
            (Audio|Components|Audio|Play (Variables|Default|GetImpactSound) 0.0)
            (Audio|Components|Audio|SetVolumeMultiplier (Variables|Default|GetImpactSound) (Math|Float|MapRangeClamped (Variables|Default|GetForce) 3e+03 1e+04 0.01 0.25) :!class /Script/Engine.AudioComponent)))
        (else
          (goto _label Reset))))
    (:then_1
      ;[1 1 1] Threshold for rolling
      (if (>= (Variables|Default|GetRotationSpeed) 2.0)
        ;[1 1 1] play rolling sound
        (Utilities|FlowControl|Sequence
          (:then_0
            (Utilities|FlowControl|DoOnce false :!label _label_2
              (:Completed
                (Audio|Components|Audio|Play _rollingsound _returnvalue_2)
                (Development|PrintString (Utilities|String|ToString(Float) _returnvalue_2) false))))
          (:then_1
            (Audio|Components|Audio|SetVolumeMultiplier _rollingsound_2 (Math|Float|MapRangeClamped (Variables|Default|GetRotationSpeed) 2.0 2.5e+02 0.0 2.0) :!class /Script/Engine.AudioComponent)
            (Audio|Components|Audio|SetPitchMultiplier _rollingsound_2 (Math|Float|MapRangeClamped (Variables|Default|GetRotationSpeed) 2.0 2.5e+02 0.95 1.1))))
        (else
          (Audio|Components|Audio|FadeOut (Variables|Default|GetRollingSound) 0.1 0.0 :!class /Script/Engine.AudioComponent)
          (goto _label_2 Reset))))))

(fn ConstructionScript)