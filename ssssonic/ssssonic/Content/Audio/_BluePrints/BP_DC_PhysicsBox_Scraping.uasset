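; Physics box Blueprint that plays impact and scraping sounds driven by its physics hits.
; Hits above a force threshold play a gated impact sound with force-scaled volume, re-armed by a weaker hit.
; Sliding speed from the mesh's velocity starts the scrape once at a random offset, then modulates its volume and pitch on each hit.
; Scraping fades out and re-arms on a slow hit or when an actor overlap ends.
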(event Collision|EventActorEndOverlap
  (params (OtherActor :type Actor%20Object%20Reference))
  (bind _scrapingsound (Variables|Default|GetScrapingSound))
  ;[1 1 1] play scraping sound
  (Audio|Components|Audio|FadeOut (Variables|Default|GetScrapingSound) 0.1 0.0 :!class /Script/Engine.AudioComponent)
  (Utilities|FlowControl|DoOnce false) ; enters at Reset
)

(event Collision|EventHit
  (params (MyComp :type Primitive%20Component%20Object%20Reference) (Other :type Actor%20Object%20Reference) (OtherComp :type Primitive%20Component%20Object%20Reference) (bSelfMoved :type Boolean) (HitLocation :type Vector :default "0, 0, 0") (HitNormal :type Vector :default "0, 0, 0") (NormalImpulse :type Vector :default "0, 0, 0") (Hit :type Hit%20Result%20Structure%20%28by%20ref%29))
  (bind _scrapingsound (Variables|Default|GetScrapingSound))
  (bind _scrapingsound_2 (Variables|Default|GetScrapingSound))
  (bind _impactsound (Variables|Default|GetImpactSound))
  ;[1 1 1] hit event - get speed
  (Variables|Default|SetForce (Math|Vector|VectorLength NormalImpulse))
  (bind _returnvalue (Physics|GetPhysicsLinearVelocity (Variables|Default|GetStaticMesh) "None"))
  (Variables|Default|SetSlidingSpeed (Math|Vector|VectorLength _returnvalue))
  (Utilities|FlowControl|Sequence
    (:then_0
      ;[1 1 1] Threshold for impacts
      (if (> (Variables|Default|GetForce) 1.2e+04)
        ;[1 1 1] play impact sound
        (|DoOnceMultiInput :!label _label
          (:A%20Out
            (Audio|Components|Audio|Play _impactsound 0.0)
            (Audio|Components|Audio|SetVolumeMultiplier _impactsound (Math|Float|MapRangeClamped (Variables|Default|GetForce) 8e+03 1.5e+04 0.1 1.0) :!class /Script/Engine.AudioComponent)))
        (else
          (goto _label Reset%20In))))
    (:then_1
      ;[1 1 1] Threshold for sliding
      (if (>= (Variables|Default|GetSlidingSpeed) 1e+01)
        ;[1 1 1] play scraping sound
        (Utilities|FlowControl|Sequence
          (:then_0
            (Utilities|FlowControl|DoOnce false :!label _label_2
              (:Completed
                (Audio|Components|Audio|Play _scrapingsound (Math|Random|RandomFloatinRange 0.0 (- (Variables|/Script/Engine.SoundBase|GetDuration (Variables|/Script/Engine.AudioComponent|GetSound _scrapingsound)) 1.0))))))
          (:then_1
            (Audio|Components|Audio|SetVolumeMultiplier _scrapingsound_2 (Math|Float|MapRangeClamped (Variables|Default|GetSlidingSpeed) 1e+01 1e+03 0.0 2.0) :!class /Script/Engine.AudioComponent)
            (Audio|Components|Audio|SetPitchMultiplier _scrapingsound_2 (Math|Float|MapRangeClamped (Variables|Default|GetSlidingSpeed) 1e+01 1e+03 0.9 1.1))))
        (else
          (Audio|Components|Audio|FadeOut (Variables|Default|GetScrapingSound) 0.1 0.0 :!class /Script/Engine.AudioComponent)
          (goto _label_2 Reset))))))

(fn ConstructionScript)