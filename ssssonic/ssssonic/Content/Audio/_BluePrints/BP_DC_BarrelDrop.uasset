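; Interactive barrel drop station that lets the player spawn barrels or pumpkins and adjust the height of a splat platform.
; Box overlap with the player opens Gates that let key presses trigger spawning at set points or platform movement, and leaving closes them.
; The platform and its legs move in fixed, clamped steps.
; BeginPlay also opens the Gates if the player already overlaps the actor.
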(event OnComponentBeginOverlap(Box)
  (params (OverlappedComponent :type Primitive%20Component%20Object%20Reference) (OtherActor :type Actor%20Object%20Reference) (OtherComp :type Primitive%20Component%20Object%20Reference) (OtherBodyIndex :type Integer) (bFromSweep :type Boolean) (SweepResult :type Hit%20Result%20Structure%20%28by%20ref%29))
  ;[1 1 1] Key inputs
  (if (== OtherActor (Game|GetPlayerCharacter 0))
    (Utilities|FlowControl|Sequence
      (:then_0
        (Utilities|FlowControl|Gate true) ; enters at Open
      )
      (:then_1
        (Utilities|FlowControl|Gate true) ; enters at Open
      )
      (:then_2
        (Utilities|FlowControl|Gate true) ; enters at Open
      )
      (:then_3
        (Utilities|FlowControl|Gate true) ; enters at Open
      ))))

(event OnComponentEndOverlap(Box)
  (params (OverlappedComponent :type Primitive%20Component%20Object%20Reference) (OtherActor :type Actor%20Object%20Reference) (OtherComp :type Primitive%20Component%20Object%20Reference) (OtherBodyIndex :type Integer))
  ;[1 1 1] Key inputs
  (if (== OtherActor (Game|GetPlayerCharacter 0))
    (Utilities|FlowControl|Sequence
      (:then_0
        (Utilities|FlowControl|Gate true) ; enters at Close
      )
      (:then_1
        (Utilities|FlowControl|Gate true) ; enters at Close
      )
      (:then_2
        (Utilities|FlowControl|Gate true) ; enters at Close
      )
      (:then_3
        (Utilities|FlowControl|Gate true) ; enters at Close
      ))))

(event Custom|SpawnPumpkin
  ;[1 1 1] Spawn
  (Game|SpawnActorfromClass "/Game/Audio/_BluePrints/BP_DC_Pumpkin.BP_DC_Pumpkin_C" (Transformation|GetWorldTransform (Variables|Default|GetPumpkinSpawnPoint)) "Undefined" 0 0))

(event Custom|RaisePlatform
  ;[1 1 1] Adjust Platform Height
  (if (< (Variables|Default|GetPlatformHeightSteps) 5)
    (Math|Integer|IncrementInt (Variables|Default|GetPlatformHeightSteps)
      (:%20%20
        (Transformation|AddLocalOffset (Variables|Default|GetSplatPlatform) "0, 0,40.000000" false false)))))

(event Custom|LowerPlatform
  ;[1 1 1] Adjust Platform Height
  (if (> (Variables|Default|GetPlatformHeightSteps) 1)
    (Math|Integer|DecrementInt (Variables|Default|GetPlatformHeightSteps)
      (:%20%20
        (Transformation|AddLocalOffset (Variables|Default|GetSplatPlatform) "0, 0,-40.000000" false false)))))

(event Custom|SpawnBarrel
  ;[1 1 1] Spawn
  (Game|SpawnActorfromClass "/Game/Audio/_BluePrints/BP_DC_Barrel.BP_DC_Barrel_C" (Transformation|GetWorldTransform (Variables|Default|GetBarrelSpawnPoint)) "Undefined" 0 0))

(event EventBeginPlay
  ;[1 1 1] Key inputs
  (for _array_element (Collision|GetOverlappingActors "/Game/FirstPersonBP/Blueprints/FirstPersonCharacter.FirstPersonCharacter_C" :!class /Script/Engine.Actor)
    (if (== (Game|GetPlayerCharacter 0) _array_element)
      (Utilities|FlowControl|Sequence
        (:then_0
          (Utilities|FlowControl|Gate true) ; enters at Open
        )
        (:then_1
          (Utilities|FlowControl|Gate true) ; enters at Open
        )
        (:then_2
          (Utilities|FlowControl|Gate true) ; enters at Open
        )
        (:then_3
          (Utilities|FlowControl|Gate true) ; enters at Open
        )))))

(event Input|KeyboardEvents|Add
  (params (Key :type Key%20Structure :default "None"))
  ;[1 1 1] Key inputs
  (:Pressed
    (Utilities|FlowControl|Gate true
      (:Exit
        (CallFunction|RaisePlatform)))))

(event Input|KeyboardEvents|Subtract
  (params (Key :type Key%20Structure :default "None"))
  ;[1 1 1] Key inputs
  (:Pressed
    (Utilities|FlowControl|Gate true
      (:Exit
        (CallFunction|LowerPlatform)))))

(event Input|KeyboardEvents|R
  (params (Key :type Key%20Structure :default "None"))
  ;[1 1 1] Key inputs
  (:Pressed
    (Development|PrintString "Hello")
    (Utilities|FlowControl|Gate true
      (:Exit
        (CallFunction|SpawnPumpkin)))))

(event Input|KeyboardEvents|E
  (params (Key :type Key%20Structure :default "None"))
  ;[1 1 1] Key inputs
  (:Pressed
    (Utilities|FlowControl|Gate true
      (:Exit
        (CallFunction|SpawnBarrel)))))

(fn ConstructionScript)