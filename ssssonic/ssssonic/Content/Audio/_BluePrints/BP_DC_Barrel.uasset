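; BP_DC_Barrel is a barrel Blueprint that plays impact sounds when it is hit.
; On Hit, it normalizes the impulse magnitude into a force value.
; It plays soft, medium and hard barrel sounds together at the hit location, each with volume read from its own float curve, crossfading layers by impact strength.
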(event Collision|EventHit
  (params (MyComp :type Primitive%20Component%20Object%20Reference) (Other :type Actor%20Object%20Reference) (OtherComp :type Primitive%20Component%20Object%20Reference) (bSelfMoved :type Boolean) (HitLocation :type Vector :default "0, 0, 0") (HitNormal :type Vector :default "0, 0, 0") (NormalImpulse :type Vector :default "0, 0, 0") (Hit :type Hit%20Result%20Structure%20%28by%20ref%29))
  (Variables|Default|SetLocation HitLocation)
  (Variables|Default|SetForce (Math|Float|NormalizetoRange (Math|Vector|VectorLength NormalImpulse) 0.0 5e+04))
  (Audio|PlaySoundatLocation "/Game/Audio/Collision/BarrelImpacts/as_pr_SC_BarrelSoft.as_pr_SC_BarrelSoft" (Variables|Default|GetLocation) "0, 0, 0" (Math|Curves|GetFloatValue (Variables|Default|GetSoft) (Variables|Default|GetForce)) 1.0 0.0 0 0 0)
  (Audio|PlaySoundatLocation "/Game/Audio/Collision/BarrelImpacts/as_pr_SC_BarrelMedium.as_pr_SC_BarrelMedium" (Variables|Default|GetLocation) "0, 0, 0" (Math|Curves|GetFloatValue (Variables|Default|GetMedium) (Variables|Default|GetForce)) 1.0 0.0 0 0 0)
  (Audio|PlaySoundatLocation "/Game/Audio/Collision/BarrelImpacts/as_pr_SC_BarrelHard.as_pr_SC_BarrelHard" (Variables|Default|GetLocation) "0, 0, 0" (Math|Curves|GetFloatValue (Variables|Default|GetHard) (Variables|Default|GetForce)) 1.0 0.0 0 0 0))

(fn ConstructionScript)