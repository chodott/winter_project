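; BP_DC_Visualiser is a debug actor that visualises Ambient Sound attenuation in-game, toggled with the V key.
; On BeginPlay it spawns a BP_DC_VisualiserSphere at every AmbientSound, sizing its inner and falloff spheres from that sound's shape extent and falloff distance.
; A FlipFlop shows or hides the stored spheres, running the audio3dvisualize console command once per visualiser inside each loop.
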(event Custom|ToggleHidden
  ;[1 1 1] toggle hidden
  (Utilities|FlowControl|FlipFlop
    (:A
      (for _array_element (Variables|Default|GetVisualisers)
        (Development|SetHiddeninGame (Variables|/Game/Audio/_BluePrints/BP_DC_VisualiserSphere.BP_DC_VisualiserSphere_C|GetInnerSphere _array_element) false false)
        (Development|ExecuteConsoleCommand "audio3dvisualize" 0)))
    (:B
      (for _array_element_2 (Variables|Default|GetVisualisers)
        (Development|SetHiddeninGame (Variables|/Game/Audio/_BluePrints/BP_DC_VisualiserSphere.BP_DC_VisualiserSphere_C|GetInnerSphere _array_element_2) true false)
        (Development|ExecuteConsoleCommand "audio3dvisualize" 0)))))

(event EventBeginPlay
  ;[1 1 1] set up
  (bind _outactors (Actor|GetAllActorsOfClass "/Script/Engine.AmbientSound"))
  (Variables|Default|SetAmbientSounds _outactors)
  (for _array_element (Variables|Default|GetAmbientSounds)
    (Variables|Default|SetSound _array_element)
    (Variables|Default|SetSoundLocation (Transformation|GetActorLocation _array_element))
    (bind _outattenuationsettings (Audio|Components|Audio|GetAttenuationSettingsToApply (Variables|/Script/Engine.AmbientSound|GetAudioComponent _array_element)))
    (Variables|Default|SetInnerRadius (.X (Math|Vector|BreakVector (.AttenuationShapeExtents (Utilities|Struct|BreakSoundAttenuationSettings _outattenuationsettings)))))
    (Variables|Default|SetFalloffDistance (.FalloffDistance (Utilities|Struct|BreakSoundAttenuationSettings _outattenuationsettings)))
    (bind _returnvalue (Game|SpawnActorfromClass "/Game/Audio/_BluePrints/BP_DC_VisualiserSphere.BP_DC_VisualiserSphere_C" (Math|Transform|MakeTransform (Variables|Default|GetSoundLocation) "0, 0, 0" "1,1,1") "Undefined" 0 0))
    (Variables|/Game/Audio/_BluePrints/BP_DC_VisualiserSphere.BP_DC_VisualiserSphere_C|SetSound _returnvalue (Variables|Default|GetSound))
    (Utilities|Array|Add (Variables|Default|GetVisualisers) _returnvalue)
    (Components|Sphere|SetSphereRadius (Variables|/Game/Audio/_BluePrints/BP_DC_VisualiserSphere.BP_DC_VisualiserSphere_C|GetInnerSphere _returnvalue) (Variables|Default|GetInnerRadius) false)
    (Components|Sphere|SetSphereRadius (Variables|/Game/Audio/_BluePrints/BP_DC_VisualiserSphere.BP_DC_VisualiserSphere_C|GetFalloffSphere _returnvalue) (Variables|Default|GetFalloffDistance) false)))

(event Input|KeyboardEvents|V
  (params (Key :type Key%20Structure :default "None"))
  ;[1 1 1] key press
  (:Pressed
    (CallFunction|ToggleHidden)))

(fn ConstructionScript)