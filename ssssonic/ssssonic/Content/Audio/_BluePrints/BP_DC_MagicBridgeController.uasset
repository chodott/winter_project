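; BP_DC_MagicBridgeController is an interaction trigger that plays an assigned Level Sequence, presumably for a magic bridge.
; A gate opened and closed by Box overlap limits the E key to when the player character is inside.
; DoOnce permits one attempt per instance, which plays only if Completed is false.
; When the sequence finishes, every controller of this class is marked Completed, blocking later plays from the others.
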(event OnComponentBeginOverlap(Box)
  (params (OverlappedComponent :type Primitive%20Component%20Object%20Reference) (OtherActor :type Actor%20Object%20Reference) (OtherComp :type Primitive%20Component%20Object%20Reference) (OtherBodyIndex :type Integer) (bFromSweep :type Boolean) (SweepResult :type Hit%20Result%20Structure%20%28by%20ref%29))
  (bind _sequence (Variables|Default|GetSequence))
  (bind _sequenceplayer (Variables|/Script/LevelSequence.LevelSequenceActor|GetSequencePlayer _sequence))
  (if (== OtherActor (Game|GetPlayerCharacter 0))
    (Utilities|FlowControl|Gate true) ; enters at Open
  ))

(event OnComponentEndOverlap(Box)
  (params (OverlappedComponent :type Primitive%20Component%20Object%20Reference) (OtherActor :type Actor%20Object%20Reference) (OtherComp :type Primitive%20Component%20Object%20Reference) (OtherBodyIndex :type Integer))
  (bind _sequence (Variables|Default|GetSequence))
  (bind _sequenceplayer (Variables|/Script/LevelSequence.LevelSequenceActor|GetSequencePlayer _sequence))
  (if (== OtherActor (Game|GetPlayerCharacter 0))
    (Utilities|FlowControl|Gate true) ; enters at Close
  ))

(event Custom|OnFinished_Event_0
  (bind _outactors (Actor|GetAllActorsOfClass "BP_DC_MagicBridgeController_C"))
  (for _array_element _outactors
    (Variables|BP_DC_MagicBridgeController_C|SetCompleted _array_element true)))

(event Input|KeyboardEvents|E
  (params (Key :type Key%20Structure :default "None"))
  (bind _sequence (Variables|Default|GetSequence))
  (bind _sequenceplayer (Variables|/Script/LevelSequence.LevelSequenceActor|GetSequencePlayer _sequence))
  (:Pressed
    (Utilities|FlowControl|Gate true
      (:Exit
        (Utilities|FlowControl|DoOnce false
          (:Completed
            (if (not (Variables|Default|GetCompleted))
              (Sequencer|Player|Play _sequenceplayer :!class /Script/MovieScene.MovieSceneSequencePlayer)
              (EventDispatchers|AssignOnFinished _sequenceplayer (delegate Custom|OnFinished_Event_0)))))))))

(fn ConstructionScript)