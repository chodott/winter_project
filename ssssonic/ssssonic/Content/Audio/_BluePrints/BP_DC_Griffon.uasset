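; Interactive griffon actor that plays animations on keys 1-4 while the player is inside its trigger box.
; A box-controlled gate passes the chosen index to AnimBP_BigGriffon, then resets it after a short delay.
; Key 4 also starts a walk, alternating between random TargetPoints tagged Front and Back.
; MoveComponentTo drives the skeletal mesh's movement and 180-degree turns, toggling the AnimBP's IsMoving flag.
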(event OnComponentBeginOverlap(Box)
  (params (OverlappedComponent :type Primitive%20Component%20Object%20Reference) (OtherActor :type Actor%20Object%20Reference) (OtherComp :type Primitive%20Component%20Object%20Reference) (OtherBodyIndex :type Integer) (bFromSweep :type Boolean) (SweepResult :type Hit%20Result%20Structure%20%28by%20ref%29))
  ;[1 1 1] Switch Anims
  (if (== OtherActor (Game|GetPlayerCharacter 0))
    (Utilities|FlowControl|Gate true) ; enters at Open
  ))

(event OnComponentEndOverlap(Box)
  (params (OverlappedComponent :type Primitive%20Component%20Object%20Reference) (OtherActor :type Actor%20Object%20Reference) (OtherComp :type Primitive%20Component%20Object%20Reference) (OtherBodyIndex :type Integer))
  ;[1 1 1] Switch Anims
  (if (== OtherActor (Game|GetPlayerCharacter 0))
    (Utilities|FlowControl|Gate true) ; enters at Close
  ))

(event Custom|StopWalking
  (bind _skeletalmeshcomponent (Variables|SkeletalMeshActor|GetSkeletalMeshComponent))
  (bind _skeletalmeshcomponent_2 (Variables|SkeletalMeshActor|GetSkeletalMeshComponent))
  (bind _destination (Variables|Default|GetDestination))
  (bind _returnvalue (Transformation|GetActorLocation _destination))
  (bind _returnvalue_2 (Transformation|GetWorldLocation _skeletalmeshcomponent_2))
  (bind _returnvalue_3 (Transformation|GetWorldRotation _skeletalmeshcomponent))
  (bind _returnvalue_4 (Math|Rotator|FindLookatRotation _returnvalue_2 _returnvalue))
  ;[1 1 1] Move to
  (if (Variables|Default|GetNeedToTurnAround)
    (Utilities|FlowControl|Sequence
      (:then_0
        (Components|MoveComponentTo (Variables|SkeletalMeshActor|GetSkeletalMeshComponent) _returnvalue (Math|Rotator|MakeRotator (.roll _returnvalue_4) (.pitch _returnvalue_4) (- (.yaw _returnvalue_4) 9e+01)) false false 6.0 false) ; enters at Stop
      )
      (:then_1
        (Variables|/Game/Audio_Demo_Assets/AnimBP_BigGriffon.AnimBP_BigGriffon_C|SetIsMoving (Variables|Default|GetAnimBP) true)
        (Components|MoveComponentTo (Variables|SkeletalMeshActor|GetSkeletalMeshComponent) (Transformation|GetWorldLocation _skeletalmeshcomponent) (Math|Rotator|MakeRotator (.roll _returnvalue_3) (.pitch _returnvalue_3) (- (.yaw _returnvalue_3) 1.8e+02)) false false 0.7 false)
        (Variables|/Game/Audio_Demo_Assets/AnimBP_BigGriffon.AnimBP_BigGriffon_C|SetIsMoving (Variables|Default|GetAnimBP) false)
        (Utilities|FlowControl|Delay 0.3)
        (Variables|Default|SetNeedToTurnAround false)))
    (else
      (Components|MoveComponentTo (Variables|SkeletalMeshActor|GetSkeletalMeshComponent) _returnvalue (Math|Rotator|MakeRotator (.roll _returnvalue_4) (.pitch _returnvalue_4) (- (.yaw _returnvalue_4) 9e+01)) false false 6.0 false) ; enters at Stop
    )))

(event Custom|Walk
  (bind _skeletalmeshcomponent (Variables|SkeletalMeshActor|GetSkeletalMeshComponent))
  (bind _returnvalue (Transformation|GetWorldRotation _skeletalmeshcomponent))
  ;[1 1 1] Move to
  (Utilities|FlowControl|FlipFlop
    (:A
      (Variables|Default|SetDestination (Utilities|Array|Get(acopy) (Variables|Default|GetFrontTargetPoints) (Math|Random|RandomInteger 3))))
    (:B
      (Variables|Default|SetNeedToTurnAround true)
      (Variables|Default|SetDestination (Utilities|Array|Get(acopy) (Variables|Default|GetBackTargetPoints) (Math|Random|RandomInteger 3)))
      (Variables|/Game/Audio_Demo_Assets/AnimBP_BigGriffon.AnimBP_BigGriffon_C|SetIsMoving (Variables|Default|GetAnimBP) true)
      (Components|MoveComponentTo (Variables|SkeletalMeshActor|GetSkeletalMeshComponent) (Transformation|GetWorldLocation _skeletalmeshcomponent) (Math|Rotator|MakeRotator (.roll _returnvalue) (.pitch _returnvalue) (- (.yaw _returnvalue) 1.8e+02)) false false 0.7 false)
      (Variables|/Game/Audio_Demo_Assets/AnimBP_BigGriffon.AnimBP_BigGriffon_C|SetIsMoving (Variables|Default|GetAnimBP) false)
      (Utilities|FlowControl|Delay 0.3)))
  (Variables|/Game/Audio_Demo_Assets/AnimBP_BigGriffon.AnimBP_BigGriffon_C|SetIsMoving (Variables|Default|GetAnimBP) true)
  (Components|MoveComponentTo (Variables|SkeletalMeshActor|GetSkeletalMeshComponent) (Transformation|GetActorLocation (Variables|Default|GetDestination)) (Math|Rotator|MakeRotator (.roll (Math|Rotator|FindLookatRotation (Transformation|GetWorldLocation (Variables|SkeletalMeshActor|GetSkeletalMeshComponent)) (Transformation|GetActorLocation (Variables|Default|GetDestination)))) (.pitch (Math|Rotator|FindLookatRotation (Transformation|GetWorldLocation (Variables|SkeletalMeshActor|GetSkeletalMeshComponent)) (Transformation|GetActorLocation (Variables|Default|GetDestination)))) (- (.yaw (Math|Rotator|FindLookatRotation (Transformation|GetWorldLocation (Variables|SkeletalMeshActor|GetSkeletalMeshComponent)) (Transformation|GetActorLocation (Variables|Default|GetDestination)))) 9e+01)) false false 6.0 false)
  (Variables|/Game/Audio_Demo_Assets/AnimBP_BigGriffon.AnimBP_BigGriffon_C|SetIsMoving (Variables|Default|GetAnimBP) false)
  (CallFunction|StopWalking))

(event EventBeginPlay
  ;[1 1 1] Setup
  (bind _asanim_bp_big_griffon (Utilities|Casting|CastToAnimBP_BigGriffon (Components|SkeletalMesh|GetAnimInstance (Variables|SkeletalMeshActor|GetSkeletalMeshComponent))))
  (Variables|Default|SetAnimBP _asanim_bp_big_griffon)
  (bind _outactors (Actor|GetAllActorsOfClass "/Script/Engine.TargetPoint"))
  (for _array_element _outactors
    (if (Actor|ActorHasTag _array_element "Front")
      (Utilities|Array|Add (Variables|Default|GetFrontTargetPoints) _array_element)
      (elif (Actor|ActorHasTag _array_element "Back")
        (Utilities|Array|Add (Variables|Default|GetBackTargetPoints) _array_element)))))

(event Input|KeyboardEvents|1
  (params (Key :type Key%20Structure :default "None"))
  ;[1 1 1] Switch Anims
  (:Pressed
    (Variables|Default|SetChosenAnim 1)
    (Utilities|FlowControl|Gate true
      (:Exit
        (Variables|/Game/Audio_Demo_Assets/AnimBP_BigGriffon.AnimBP_BigGriffon_C|SetAnim (Variables|Default|GetAnimBP) (Variables|Default|GetChosenAnim))
        (Utilities|FlowControl|Delay 0.2)
        (Variables|/Game/Audio_Demo_Assets/AnimBP_BigGriffon.AnimBP_BigGriffon_C|SetAnim (Variables|Default|GetAnimBP) 0)
        (if (not (!= (Variables|Default|GetChosenAnim) 4))
          (CallFunction|Walk))))))

(event Input|KeyboardEvents|2
  (params (Key :type Key%20Structure :default "None"))
  ;[1 1 1] Switch Anims
  (:Pressed
    (Variables|Default|SetChosenAnim 2)
    (Utilities|FlowControl|Gate true
      (:Exit
        (Variables|/Game/Audio_Demo_Assets/AnimBP_BigGriffon.AnimBP_BigGriffon_C|SetAnim (Variables|Default|GetAnimBP) (Variables|Default|GetChosenAnim))
        (Utilities|FlowControl|Delay 0.2)
        (Variables|/Game/Audio_Demo_Assets/AnimBP_BigGriffon.AnimBP_BigGriffon_C|SetAnim (Variables|Default|GetAnimBP) 0)
        (if (not (!= (Variables|Default|GetChosenAnim) 4))
          (CallFunction|Walk))))))

(event Input|KeyboardEvents|3
  (params (Key :type Key%20Structure :default "None"))
  ;[1 1 1] Switch Anims
  (:Pressed
    (Variables|Default|SetChosenAnim 3)
    (Utilities|FlowControl|Gate true
      (:Exit
        (Variables|/Game/Audio_Demo_Assets/AnimBP_BigGriffon.AnimBP_BigGriffon_C|SetAnim (Variables|Default|GetAnimBP) (Variables|Default|GetChosenAnim))
        (Utilities|FlowControl|Delay 0.2)
        (Variables|/Game/Audio_Demo_Assets/AnimBP_BigGriffon.AnimBP_BigGriffon_C|SetAnim (Variables|Default|GetAnimBP) 0)
        (if (not (!= (Variables|Default|GetChosenAnim) 4))
          (CallFunction|Walk))))))

(event Input|KeyboardEvents|4
  (params (Key :type Key%20Structure :default "None"))
  ;[1 1 1] Switch Anims
  (:Pressed
    (Variables|Default|SetChosenAnim 4)
    (Utilities|FlowControl|Gate true
      (:Exit
        (Variables|/Game/Audio_Demo_Assets/AnimBP_BigGriffon.AnimBP_BigGriffon_C|SetAnim (Variables|Default|GetAnimBP) (Variables|Default|GetChosenAnim))
        (Utilities|FlowControl|Delay 0.2)
        (Variables|/Game/Audio_Demo_Assets/AnimBP_BigGriffon.AnimBP_BigGriffon_C|SetAnim (Variables|Default|GetAnimBP) 0)
        (if (not (!= (Variables|Default|GetChosenAnim) 4))
          (CallFunction|Walk))))))

(fn ConstructionScript)