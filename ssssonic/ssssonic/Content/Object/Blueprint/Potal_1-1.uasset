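; Portal actor that moves whatever hits it to a stored destination, P12Position, by setting the other actor's root component location without sweep.
; A CoolTime flag is set after each move, so a later hit waits through a three-second delay before it clears the flag and still teleports.
; BeginPlay records the mesh's own location as P11Position; this graph never assigns the destination.
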(event EventBeginPlay
  (Variables|Default|SetP_1-1_position (Transformation|GetWorldLocation (Variables|Debug|GetStaticMeshComponent))))

(event Collision|EventHit
  (params (MyComp :type Primitive%20Component%20Object%20Reference) (Other :type Actor%20Object%20Reference) (OtherComp :type Primitive%20Component%20Object%20Reference) (bSelfMoved :type Boolean) (HitLocation :type Vector :default "0, 0, 0") (HitNormal :type Vector :default "0, 0, 0") (NormalImpulse :type Vector :default "0, 0, 0") (Hit :type Hit%20Result%20Structure%20%28by%20ref%29))
  (if (Variables|Default|GetCoolTime)
    (Utilities|FlowControl|Delay 3.0)
    (Variables|Default|SetCoolTime false))
  (Transformation|SetWorldLocation (Variables|/Script/Engine.Actor|GetRootComponent Other) (Variables|Default|GetP_1-2_position) false false)
  (Variables|Default|SetCoolTime true))

(fn ConstructionScript)