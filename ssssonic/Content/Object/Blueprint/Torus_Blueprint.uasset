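; Torus actor that, once another actor overlaps it, expands horizontally and then disappears.
; The overlap event sets an Active flag, which lets Tick add a fixed step to the X and Y scale each frame, independent of delta time.
; The actor destroys itself when the length of its scale vector passes a threshold.
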(event EventBeginPlay)

(event EventTick
  (params (DeltaSeconds :type Float%20%28single-precision%29))
  (bind _returnvalue (Transformation|GetActorScale3D))
  (if (Variables|Default|Getactive)
    (Transformation|SetActorScale3D (+ _returnvalue "0.200000,0.200000, 0"))
    (if (> (Math|Vector|VectorLength _returnvalue) 5.0)
      (Actor|DestroyActor))))

(event Collision|EventActorBeginOverlap
  (params (OtherActor :type Actor%20Object%20Reference))
  (Variables|Default|Setactive true))

(fn ConstructionScript)